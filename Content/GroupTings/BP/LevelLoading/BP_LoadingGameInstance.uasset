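; Game instance that handles loading screen transitions and player start.
; LoadingScreenFadeIn shows a fade-in widget, waits for its animation length plus FadeDelay, then opens the LoadingScreen level.
; LoadingScreenFadeOut shows a fade-out widget and removes it once the animation length has elapsed.
; StartPlayer restarts player 0 through the game mode, sets game-only input and hides the mouse cursor.
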(event Custom|LoadingScreenFadeIn
  (bind _returnvalue (UserInterface|CreateWidget "/Game/GroupTings/BP/UI/LoadingScreen/WBP_LoadingScreenFadeIn.WBP_LoadingScreenFadeIn_C"))
  (UserInterface|Viewport|AddtoViewport _returnvalue 2)
  (Utilities|FlowControl|Delay (+ (Class|WidgetAnimation|GetEndTime (Variables|/Game/GroupTings/BP/UI/LoadingScreen/WBP_LoadingScreenFadeIn.WBP_LoadingScreenFadeIn_C|GetFadeIn _returnvalue)) (Variables|Default|GetfadeDelay)))
  (Game|OpenLevel(byObjectReference) "/Game/GroupTings/Levels/LoadingScreen.LoadingScreen"))

(event Custom|LoadingScreenFadeOut
  (bind _returnvalue (UserInterface|CreateWidget "/Game/GroupTings/BP/UI/LoadingScreen/WBP_LoadingScreenFadeOut.WBP_LoadingScreenFadeOut_C"))
  (UserInterface|Viewport|AddtoViewport _returnvalue 2)
  (Utilities|FlowControl|Delay (Class|WidgetAnimation|GetEndTime (Variables|/Game/GroupTings/BP/UI/LoadingScreen/WBP_LoadingScreenFadeOut.WBP_LoadingScreenFadeOut_C|GetFadeOut _returnvalue)))
  (Widget|RemovefromParent _returnvalue))

(fn StartPlayer
  (bind _returnvalue (Game|GetPlayerController 0))
  (Class|GameModeBase|RestartPlayer (Game|GetGameMode) (Game|GetPlayerController 0))
  (Input|SetInputModeGameOnly _returnvalue)
  (Variables|/Script/Engine.PlayerController|SetbShowMouseCursor _returnvalue false))