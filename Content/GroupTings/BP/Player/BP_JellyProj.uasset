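; BP_JellyProj is a jelly projectile that turns into an interactable jelly once it comes to rest.
; When its projectile movement stops, it spawns a BP_Jelly at the mesh transform and destroys itself.
; On hit, it pushes physics-simulating components with an impulse at its own location, scaled from its velocity by ImpulseForce.
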(event OnProjectileStop(ProjectileMovement)
  (params (ImpactResult :type Hit%20Result%20Structure%20%28by%20ref%29))
  ;[1 1 1] Replace projectile with an interactable jelly when the projectile is not moving anymore
  (Components|Activation|Deactivate (Variables|Default|GetProjectileMovement))
  (Game|SpawnActorfromClass "/Game/GroupTings/BP/Interactable/BP_Jelly.BP_Jelly_C" (Transformation|GetWorldTransform (Variables|Default|GetMesh)) "Undefined" 0 0)
  (Actor|DestroyActor))

(event Collision|EventHit
  (params (MyComp :type Primitive%20Component%20Object%20Reference) (Other :type Actor%20Object%20Reference) (OtherComp :type Primitive%20Component%20Object%20Reference) (bSelfMoved :type Boolean) (HitLocation :type Vector :default "0, 0, 0") (HitNormal :type Vector :default "0, 0, 0") (NormalImpulse :type Vector :default "0, 0, 0") (Hit :type Hit%20Result%20Structure%20%28by%20ref%29))
  (if (Physics|IsSimulatingPhysics OtherComp "None")
    (Physics|AddImpulseatLocation OtherComp (* (Variables|/Script/Engine.MovementComponent|GetVelocity (Variables|Default|GetProjectileMovement)) (Variables|Default|GetimpulseForce)) (Transformation|GetActorLocation) "None")))

(fn ConstructionScript)