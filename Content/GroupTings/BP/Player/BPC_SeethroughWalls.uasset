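; BPC_SeethroughWalls is a component that keeps the jelly player visible when something blocks the camera's view of it.
; Each tick, HighLightObject sphere-traces from the follow camera to the player's head on the Visibility channel and enables custom depth on the player mesh while the trace hits.
; An alternative OccludeObjects function, not called here, eases a Radius parameter in MPC_Occlusion based on a similar trace.
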(event EventTick
  (params (DeltaSeconds :type Float%20%28single-precision%29))
  (bind _returnvalue (Game|GetPlayerCharacter 0))
  (Utilities|IsValid _returnvalue
    (:Is%20Valid
      (bind _asbp_player_jelly (Utilities|Casting|CastToBP_PlayerJelly _returnvalue))
      (CallFunction|HighLightObject (Transformation|GetWorldLocation (Variables|/Game/GroupTings/BP/Player/BP_PlayerJelly.BP_PlayerJelly_C|GetFollowCamera _asbp_player_jelly)) (Transformation|GetWorldLocation (Variables|/Game/GroupTings/BP/Player/BP_PlayerJelly.BP_PlayerJelly_C|Gethead _asbp_player_jelly)) (Variables|/Game/GroupTings/BP/Player/BP_PlayerJelly.BP_PlayerJelly_C|GetrayCastRadius _asbp_player_jelly)))))

(fn OccludeObjects
  (params (cameraPosition :type Vector) (targetPosition :type Vector) (radius :type Float%20%28double-precision%29))
  (bind _returnvalue (Collision|SphereTraceByChannel cameraPosition targetPosition radius "TraceTypeQuery1" false 0 "None"))
  (bind _output_get (Variables|Default|Setradius (Math|Float|SelectFloat (Math|Interpolation|FInterpTo (Variables|Default|Getradius) (Variables|Default|GetocclusionRadius) (Utilities|Time|GetWorldDeltaSeconds) (Variables|Default|GetradiusLerpSpeed)) (Math|Interpolation|FInterpTo (Variables|Default|Getradius) 0.0 (Utilities|Time|GetWorldDeltaSeconds) (Variables|Default|GetradiusLerpSpeed)) _returnvalue)))
  (Rendering|Material|SetScalarParameterValue "/Game/GroupTings/Materials/Occlusion/MPC_Occlusion.MPC_Occlusion" "Radius" _output_get :!class /Script/Engine.KismetMaterialLibrary))

(fn HighLightObject
  (params (cameraPosition :type Vector) (targetPosition :type Vector) (radius :type Float%20%28double-precision%29))
  (bind _returnvalue (Game|GetPlayerCharacter 0))
  (bind _returnvalue_2 (Collision|SphereTraceByChannel cameraPosition targetPosition radius "TraceTypeQuery1" false 0 "None"))
  (Utilities|IsValid _returnvalue
    (:Is%20Valid
      (bind _asbp_player_jelly (Utilities|Casting|CastToBP_PlayerJelly _returnvalue))
      (if _returnvalue_2
        (Rendering|SetRenderCustomDepth (Variables|/Script/Engine.Character|GetMesh _asbp_player_jelly) true)
        (else
          (Rendering|SetRenderCustomDepth (Variables|/Script/Engine.Character|GetMesh _asbp_player_jelly) false))))))