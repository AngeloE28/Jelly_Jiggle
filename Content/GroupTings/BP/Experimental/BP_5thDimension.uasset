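; BP_5thDimension is an experimental trigger that switches a stencil-based visibility state based on which side the player enters from.
; When any Character begins overlapping, it dots its forward vector with the direction to player 0.
; In front, it sets Stencil_ID to 1 on BP_PlayerJelly's material and shows its static mesh in game.
; Otherwise, it resets the ID to 0 and hides the mesh.
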(event Collision|EventActorBeginOverlap
  (params (OtherActor :type Actor%20Object%20Reference))
  (bind _returnvalue (Game|GetPlayerCharacter 0))
  (if (Utilities|ClassIsChildOf (Utilities|GetClass OtherActor) "/Script/Engine.Character")
    (Utilities|IsValid _returnvalue
      (:Is%20Valid
        (if (> (Math|Vector|DotProduct (Math|Vector|Normalize (Transformation|GetActorForwardVector)) (Math|Vector|Normalize (- (Transformation|GetActorLocation _returnvalue) (Transformation|GetActorLocation)))) 0.0)
          (bind _asbp_player_jelly (Utilities|Casting|CastToBP_PlayerJelly _returnvalue))
          (Rendering|Material|SetScalarParameterValue (Variables|/Game/GroupTings/BP/Player/BP_PlayerJelly.BP_PlayerJelly_C|GetJellyMaterial _asbp_player_jelly) "Stencil_ID" 1.0 :!class /Script/Engine.MaterialInstanceDynamic)
          (Development|SetHiddeninGame (Variables|Debug|GetStaticMeshComponent) false false)
          (else
            (bind _asbp_player_jelly_2 (Utilities|Casting|CastToBP_PlayerJelly _returnvalue))
            (Rendering|Material|SetScalarParameterValue (Variables|/Game/GroupTings/BP/Player/BP_PlayerJelly.BP_PlayerJelly_C|GetJellyMaterial _asbp_player_jelly_2) "Stencil_ID" 0.0 :!class /Script/Engine.MaterialInstanceDynamic)
            (Development|SetHiddeninGame (Variables|Debug|GetStaticMeshComponent) true false)))))))

(fn ConstructionScript)