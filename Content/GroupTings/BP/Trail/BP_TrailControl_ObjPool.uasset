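; Trail controller that lays decals behind the player jelly as it moves, sized by the jelly's raycast mesh radius.
; A looping timer adds a point and decal beyond a distance threshold, tracking them in parallel arrays.
; Each point's lifetime counts up to a maximum, then down to zero before removal, sparing the newest.
; Despite the ObjPool name, decals are spawned and destroyed, and the scaling logic is disconnected.
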(event Custom|DecalLoop
  (bind _pointlocationarray (Variables|ApplicationVariables|GetPointLocationArray))
  (Variables|ApplicationVariables|SetPlayerLocationCurrent (Transformation|GetActorLocation (Game|GetPlayerCharacter 0)))
  (if (>= (Math|Vector|VectorLength (- (Variables|ApplicationVariables|GetPlayerLocationCurrent) (Utilities|Array|Get(acopy) _pointlocationarray (Utilities|Array|LastIndex _pointlocationarray)))) (Variables|ApplicationVariables|GetDistanceThresholdToAddNewPoint))
    (Utilities|Array|Add (Variables|ApplicationVariables|GetPointLocationArray) (Variables|ApplicationVariables|GetPlayerLocationCurrent))
    (Utilities|Array|Add (Variables|ApplicationVariables|GetPointCurrentLifetimes) 0.0)
    (Utilities|Array|Add (Variables|ApplicationVariables|GetHasItReachedMaxSizeYet) false)
    (Collision|LineTraceForObjects (Variables|ApplicationVariables|GetPlayerLocationCurrent) (Math|Vector|MakeVector (.X (Math|Vector|BreakVector (Variables|ApplicationVariables|GetPlayerLocationCurrent))) (.Y (Math|Vector|BreakVector (Variables|ApplicationVariables|GetPlayerLocationCurrent))) -1.5e+02) (Utilities|Array|MakeArray "ObjectTypeQuery1") false (Utilities|Array|MakeArray (Game|GetPlayerController 0)) "None")
    (bind _asbp_player_jelly (Utilities|Casting|CastToBP_PlayerJelly (Game|Player|GetPlayerPawn 0)))
    (bind _returnvalue (Rendering|Decal|SpawnDecalatLocation (Variables|ApplicationVariables|GetDecalMaterial) (* (Variables|ApplicationVariables|GetDefaultDecalSize) (Variables|/Game/GroupTings/BP/Player/BP_PlayerJelly.BP_PlayerJelly_C|GetrayCastRadius%28JellyMeshSize%29 _asbp_player_jelly)) (Transformation|GetActorLocation (Game|GetPlayerCharacter 0)) "-90.000000,0.000000,0.000000" 5.0))
    (Variables|Default|SetMostRecentDecal _returnvalue)
    (Utilities|Array|Add (Variables|ApplicationVariables|GetArrayOfDecals) _returnvalue))
  (bind (_arrayindex _arrayelement) (Utilities|Array|ReverseforEachLoop (Variables|ApplicationVariables|GetPointCurrentLifetimes))
    (:LoopBody
      (Variables|ApplicationVariables|SetCurrentIndex _arrayindex)
      (if (Utilities|Array|Get(acopy) (Variables|ApplicationVariables|GetHasItReachedMaxSizeYet) _arrayindex)
        (if (!= (Utilities|Array|Get(acopy) (Variables|ApplicationVariables|GetArrayOfDecals) (Variables|ApplicationVariables|GetCurrentIndex)) (Variables|Default|GetMostRecentDecal))
          (Utilities|Array|SetArrayElem (Variables|ApplicationVariables|GetPointCurrentLifetimes) (Variables|ApplicationVariables|GetCurrentIndex) (- _arrayelement (Variables|Default|GettimerTick)))
          (if (<= (Utilities|Array|Get(acopy) (Variables|ApplicationVariables|GetPointCurrentLifetimes) (Variables|ApplicationVariables|GetCurrentIndex)) 0.0)
            (Utilities|Array|SetArrayElem (Variables|ApplicationVariables|GetPointCurrentLifetimes) (Variables|ApplicationVariables|GetCurrentIndex) 0.0)))
        (else
          (Utilities|Array|SetArrayElem (Variables|ApplicationVariables|GetPointCurrentLifetimes) (Variables|ApplicationVariables|GetCurrentIndex) (+ _arrayelement (Variables|Default|GettimerTick)))
          (if (>= (Utilities|Array|Get(acopy) (Variables|ApplicationVariables|GetPointCurrentLifetimes) (Variables|ApplicationVariables|GetCurrentIndex)) (Variables|ApplicationVariables|GetMaxPointLifetime))
            (Utilities|Array|SetArrayElem (Variables|ApplicationVariables|GetPointCurrentLifetimes) (Variables|ApplicationVariables|GetCurrentIndex) (Variables|ApplicationVariables|GetMaxPointLifetime))
            (if (!= (Utilities|Array|Get(acopy) (Variables|ApplicationVariables|GetArrayOfDecals) (Variables|ApplicationVariables|GetCurrentIndex)) (Variables|Default|GetMostRecentDecal))
              (Utilities|Array|SetArrayElem (Variables|ApplicationVariables|GetHasItReachedMaxSizeYet) (Variables|ApplicationVariables|GetCurrentIndex) true))))))
    (:Completed
      (bind (_arrayindex_2 _arrayelement_2) (Utilities|Array|ReverseforEachLoop (Variables|ApplicationVariables|GetHasItReachedMaxSizeYet))
        (:LoopBody
          (Variables|ApplicationVariables|SetCurrentIndex _arrayindex_2)
          (if (Math|Boolean|ANDBoolean _arrayelement_2 (!= (Utilities|Array|Get(acopy) (Variables|ApplicationVariables|GetArrayOfDecals) (Variables|ApplicationVariables|GetCurrentIndex)) (Variables|Default|GetMostRecentDecal)) (> (Utilities|Array|Length (Variables|ApplicationVariables|GetHasItReachedMaxSizeYet)) 1) (<= (Utilities|Array|Get(acopy) (Variables|ApplicationVariables|GetPointCurrentLifetimes) _arrayindex_2) 0.0))
            (Components|DestroyComponent (Utilities|Array|Get(acopy) (Variables|ApplicationVariables|GetArrayOfDecals) (Variables|ApplicationVariables|GetCurrentIndex)))
            (Utilities|Array|RemoveIndex (Variables|ApplicationVariables|GetArrayOfDecals) (Variables|ApplicationVariables|GetCurrentIndex))
            (Utilities|Array|RemoveIndex (Variables|ApplicationVariables|GetPointLocationArray) (Variables|ApplicationVariables|GetCurrentIndex))
            (Utilities|Array|RemoveIndex (Variables|ApplicationVariables|GetPointCurrentLifetimes) (Variables|ApplicationVariables|GetCurrentIndex))
            (Utilities|Array|RemoveIndex (Variables|ApplicationVariables|GetHasItReachedMaxSizeYet) (Variables|ApplicationVariables|GetCurrentIndex))))))))

(event EventBeginPlay
  (bind _returnvalue (Game|GetPlayerController 0))
  (bind _returnvalue_2 (Game|GetPlayerController 0))
  (bind _returnvalue_3 (Transformation|GetActorLocation _returnvalue))
  (bind _returnvalue_4 (Transformation|GetActorLocation _returnvalue_2))
  (bind (_x _y) (Math|Vector|BreakVector _returnvalue_4))
  (Variables|ApplicationVariables|SetPlayerLocationCurrent _returnvalue_3)
  (Utilities|Array|Add (Variables|ApplicationVariables|GetPointLocationArray) _returnvalue_3)
  (Utilities|Array|Add (Variables|ApplicationVariables|GetPointCurrentLifetimes) 0.0)
  (Utilities|Array|Add (Variables|ApplicationVariables|GetHasItReachedMaxSizeYet) false)
  (bind _outhit (Collision|LineTraceForObjects _returnvalue_4 (Math|Vector|MakeVector _x _y -1.5e+02) (Utilities|Array|MakeArray "ObjectTypeQuery1") false (Utilities|Array|MakeArray (Game|GetPlayerController 0)) "None"))
  (bind _asbp_player_jelly (Utilities|Casting|CastToBP_PlayerJelly (Game|Player|GetPlayerPawn 0)))
  (bind _returnvalue_5 (Rendering|Decal|SpawnDecalatLocation (Variables|ApplicationVariables|GetDecalMaterial) (* (Variables|ApplicationVariables|GetDefaultDecalSize) (Variables|/Game/GroupTings/BP/Player/BP_PlayerJelly.BP_PlayerJelly_C|GetrayCastRadius%28JellyMeshSize%29 _asbp_player_jelly)) (.Location (Collision|BreakHitResult _outhit)) "-90.000000,0.000000,0.000000" 5.0))
  (Variables|Default|SetMostRecentDecal _returnvalue_5)
  (Utilities|Array|Add (Variables|ApplicationVariables|GetArrayOfDecals) 0)
  (Utilities|Time|SetTimerbyEvent (delegate Custom|DecalLoop) 0.05 true))

(fn ConstructionScript)