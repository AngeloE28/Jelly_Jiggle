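; Object pool actor for decal actors, apparently for a trail effect, that reuses spawned instances.
; On BeginPlay, or when J is pressed, it spawns a batch sized by MaxPoolSize at the Box's transform.
; GetPooledObject teleports the first pooled actor to a requested transform, with no growth when empty.
; ReturnObjectToPool parks actors back at the Box and re-adds them, leaving decals visible throughout.
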(event Custom|ReturnObjectToPool
  (params (Decal :type Decal%20Actor%20Object%20Reference))
  (bind _output_get (Variables|Default|SetReturnObject Decal))
  (Development|SetHiddeninGame (Variables|/Script/Engine.DecalActor|GetDecal _output_get) false true)
  (Transformation|SetActorTransform (Variables|Default|GetReturnObject) (Variables|Default|GetPoolTransform) false true)
  (Utilities|Array|Add (Variables|Default|GetPool) (Variables|Default|GetReturnObject)))

(event EventBeginPlay
  (Variables|Default|SetPoolTransform (Transformation|GetWorldTransform (Variables|Default|GetBox)))
  (for _index (range 0 (- (Variables|Default|GetMaxPoolSize) 0))
    (bind _returnvalue (Game|SpawnActorfromClass (Variables|Default|GetClassToSpawn) (Variables|Default|GetPoolTransform) "Undefined" 0 0))
    (Utilities|Array|Add (Variables|Default|GetPool) _returnvalue)
    (Development|SetHiddeninGame (Variables|/Script/Engine.DecalActor|GetDecal _returnvalue) false true)))

(event Input|KeyboardEvents|J
  (params (Key :type Key%20Structure :default "None"))
  (:Pressed
    (Variables|Default|SetPoolTransform (Transformation|GetWorldTransform (Variables|Default|GetBox)))
    (for _index (range 0 (- (Variables|Default|GetMaxPoolSize) 0))
      (bind _returnvalue (Game|SpawnActorfromClass (Variables|Default|GetClassToSpawn) (Variables|Default|GetPoolTransform) "Undefined" 0 0))
      (Utilities|Array|Add (Variables|Default|GetPool) _returnvalue)
      (Development|SetHiddeninGame (Variables|/Script/Engine.DecalActor|GetDecal _returnvalue) false true))))

(fn ConstructionScript)

(fn GetPooledObject
  (params (Transform :type Transform))
  (bind _pool (Variables|Default|GetPool))
  (if (> (Utilities|Array|Length _pool) 0)
    (bind _output_get (Variables|Default|SetPooledObject (Utilities|Array|Get(acopy) _pool)))
    (Utilities|Array|RemoveItem (Variables|Default|GetPool) _output_get)
    (Transformation|SetActorTransform (Variables|Default|GetPooledObject) Transform false true)
    (Development|SetHiddeninGame (Variables|/Script/Engine.DecalActor|GetDecal (Variables|Default|GetPooledObject)) false true)
    (return (Variables|Default|GetPooledObject))))