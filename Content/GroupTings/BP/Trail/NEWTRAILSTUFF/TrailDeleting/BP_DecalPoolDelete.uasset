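; An object pool actor for decals, apparently used for the player jelly's trail.
; On BeginPlay it spawns hidden decal actors at offset positions from its Box and stores them in an array.
; GetPooledObject takes the first entry, moves it to a given transform and shows it.
; ReturnObjectToPool re-adds a decal but leaves it visible, teleporting it to the player jelly with scale derived from its capsule.
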(event Custom|ReturnObjectToPool
  (params (Decal :type Decal%20Actor%20Object%20Reference))
  (bind _output_get (Variables|Default|SetReturnObject Decal))
  (Rendering|SetVisibility (Variables|/Script/Engine.DecalActor|GetDecal _output_get) true true)
  (bind _asbp_player_jelly (Utilities|Casting|CastToBP_PlayerJelly (Game|Player|GetPlayerPawn 0)))
  (Transformation|SetActorTransform (Variables|Default|GetReturnObject) (Math|Transform|MakeTransform (Transformation|GetActorLocation _asbp_player_jelly) "-90.000000, 0, 0" (/ (Transformation|GetWorldScale (Variables|/Script/Engine.Character|GetCapsuleComponent _asbp_player_jelly)) "3.000000,3.000000,3.000000")) false true)
  (Utilities|Array|Add (Variables|Default|GetPool) (Variables|Default|GetReturnObject)))

(event EventBeginPlay
  (Variables|Default|SetPoolTransform (Transformation|GetWorldTransform (Variables|Default|GetBox)))
  (for _index (range 0 (- (Variables|Default|GetMaxPoolSize) 0))
    (bind _returnvalue (Game|SpawnActorfromClass (Variables|Default|GetClassToSpawn) (Variables|Default|GetPoolTransform) "Undefined" 0 0))
    (Utilities|Array|Add (Variables|Default|GetPool) _returnvalue)
    (Rendering|SetVisibility (Variables|/Script/Engine.DecalActor|GetDecal _returnvalue) false true)
    (Variables|Default|SetPoolTransform (Math|Transform|MakeTransform (+ (.location (Variables|Default|GetPoolTransform)) "10.000000,10.000000,0.000000") (.rotation (Variables|Default|GetPoolTransform)) (.scale (Variables|Default|GetPoolTransform))))))

(fn ConstructionScript)

(fn GetPooledObject
  (params (Transform :type Transform))
  (bind _pool (Variables|Default|GetPool))
  (if (> (Utilities|Array|Length _pool) 0)
    (bind _output_get (Variables|Default|SetPooledObject (Utilities|Array|Get(acopy) _pool)))
    (Utilities|Array|RemoveItem (Variables|Default|GetPool) _output_get)
    (Transformation|SetActorTransform (Variables|Default|GetPooledObject) Transform false true)
    (Rendering|SetVisibility (Variables|/Script/Engine.DecalActor|GetDecal (Variables|Default|GetPooledObject)) true true)
    (return (Variables|Default|GetPooledObject))))