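; Trail controller that drops decals behind the player jelly as it moves, sized by the jelly's mesh-radius value.
; A looping timer adds a decal whenever the player moves past a distance threshold from the last point.
; Parallel arrays track each point's lifetime, which counts up to a maximum then down before removal, sparing the newest decal.
; Decals also have a fixed lifespan, and the lifetime-based scaling logic is unconnected.
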(event Custom|DecalLoop
  (bind _pointlocationarray (Variables|Default|GetPointLocationArray))
  (Variables|Default|SetPlayerLocationCurrent (Transformation|GetActorLocation (Game|GetPlayerCharacter 0)))
  (if (>= (Math|Vector|VectorLength (- (Variables|Default|GetPlayerLocationCurrent) (Utilities|Array|Get(acopy) _pointlocationarray (Utilities|Array|LastIndex _pointlocationarray)))) (Variables|Default|GetDistanceThresholdToAddNewPoint))
    (Utilities|Array|Add (Variables|Default|GetPointLocationArray) (Variables|Default|GetPlayerLocationCurrent))
    (Utilities|Array|Add (Variables|Default|GetPointCurrentLifetimes) 0.0)
    (Utilities|Array|Add (Variables|Default|GetHasItReachedMaxSizeYet) false)
    (Collision|LineTraceForObjects (Variables|Default|GetPlayerLocationCurrent) (Math|Vector|MakeVector (.X (Math|Vector|BreakVector (Variables|Default|GetPlayerLocationCurrent))) (.Y (Math|Vector|BreakVector (Variables|Default|GetPlayerLocationCurrent))) -1.5e+02) (Utilities|Array|MakeArray "ObjectTypeQuery1") false (Utilities|Array|MakeArray (Game|GetPlayerController 0)) "None")
    (bind _asbp_player_jelly (Utilities|Casting|CastToBP_PlayerJelly (Game|Player|GetPlayerPawn 0)))
    (bind _returnvalue (Rendering|Decal|SpawnDecalatLocation (Variables|Default|GetDecalMaterial) (* (Variables|Default|GetDefaultDecalSize) (Variables|/Game/GroupTings/BP/Player/BP_PlayerJelly.BP_PlayerJelly_C|GetrayCastRadius%28JellyMeshSize%29 _asbp_player_jelly)) (Transformation|GetActorLocation (Game|GetPlayerCharacter 0)) "-90.000000,0.000000,0.000000" 5.0))
    (Variables|Default|SetMostRecentDecal _returnvalue)
    (Utilities|Array|Add (Variables|Default|GetArrayOfDecals) _returnvalue))
  (bind (_arrayindex _arrayelement) (Utilities|Array|ReverseforEachLoop (Variables|Default|GetPointCurrentLifetimes))
    (:LoopBody
      (Variables|Default|SetCurrentIndex _arrayindex)
      (if (Utilities|Array|Get(acopy) (Variables|Default|GetHasItReachedMaxSizeYet) _arrayindex)
        (if (!= (Utilities|Array|Get(acopy) (Variables|Default|GetArrayOfDecals) (Variables|Default|GetCurrentIndex)) (Variables|Default|GetMostRecentDecal))
          (Utilities|Array|SetArrayElem (Variables|Default|GetPointCurrentLifetimes) (Variables|Default|GetCurrentIndex) (- _arrayelement (Variables|Default|GettimerTick)))
          (if (<= (Utilities|Array|Get(acopy) (Variables|Default|GetPointCurrentLifetimes) (Variables|Default|GetCurrentIndex)) 0.0)
            (Utilities|Array|SetArrayElem (Variables|Default|GetPointCurrentLifetimes) (Variables|Default|GetCurrentIndex) 0.0)))
        (else
          (Utilities|Array|SetArrayElem (Variables|Default|GetPointCurrentLifetimes) (Variables|Default|GetCurrentIndex) (+ _arrayelement (Variables|Default|GettimerTick)))
          (if (>= (Utilities|Array|Get(acopy) (Variables|Default|GetPointCurrentLifetimes) (Variables|Default|GetCurrentIndex)) (Variables|Default|GetMaxPointLifetime))
            (Utilities|Array|SetArrayElem (Variables|Default|GetPointCurrentLifetimes) (Variables|Default|GetCurrentIndex) (Variables|Default|GetMaxPointLifetime))
            (if (!= (Utilities|Array|Get(acopy) (Variables|Default|GetArrayOfDecals) (Variables|Default|GetCurrentIndex)) (Variables|Default|GetMostRecentDecal))
              (Utilities|Array|SetArrayElem (Variables|Default|GetHasItReachedMaxSizeYet) (Variables|Default|GetCurrentIndex) true))))))
    (:Completed
      (bind (_arrayindex_2 _arrayelement_2) (Utilities|Array|ReverseforEachLoop (Variables|Default|GetHasItReachedMaxSizeYet))
        (:LoopBody
          (Variables|Default|SetCurrentIndex _arrayindex_2)
          (if (Math|Boolean|ANDBoolean _arrayelement_2 (!= (Utilities|Array|Get(acopy) (Variables|Default|GetArrayOfDecals) (Variables|Default|GetCurrentIndex)) (Variables|Default|GetMostRecentDecal)) (> (Utilities|Array|Length (Variables|Default|GetHasItReachedMaxSizeYet)) 1) (<= (Utilities|Array|Get(acopy) (Variables|Default|GetPointCurrentLifetimes) _arrayindex_2) 0.0))
            (Components|DestroyComponent (Utilities|Array|Get(acopy) (Variables|Default|GetArrayOfDecals) (Variables|Default|GetCurrentIndex)))
            (Utilities|Array|RemoveIndex (Variables|Default|GetArrayOfDecals) (Variables|Default|GetCurrentIndex))
            (Utilities|Array|RemoveIndex (Variables|Default|GetPointLocationArray) (Variables|Default|GetCurrentIndex))
            (Utilities|Array|RemoveIndex (Variables|Default|GetPointCurrentLifetimes) (Variables|Default|GetCurrentIndex))
            (Utilities|Array|RemoveIndex (Variables|Default|GetHasItReachedMaxSizeYet) (Variables|Default|GetCurrentIndex))))))))

(event EventBeginPlay
  (bind _returnvalue (Game|GetPlayerController 0))
  (bind _returnvalue_2 (Game|GetPlayerController 0))
  (bind _returnvalue_3 (Transformation|GetActorLocation _returnvalue))
  (bind _returnvalue_4 (Transformation|GetActorLocation _returnvalue_2))
  (bind (_x _y) (Math|Vector|BreakVector _returnvalue_4))
  (Variables|Default|SetPlayerLocationCurrent _returnvalue_3)
  (Utilities|Array|Add (Variables|Default|GetPointLocationArray) _returnvalue_3)
  (Utilities|Array|Add (Variables|Default|GetPointCurrentLifetimes) 0.0)
  (Utilities|Array|Add (Variables|Default|GetHasItReachedMaxSizeYet) false)
  (bind _outhit (Collision|LineTraceForObjects _returnvalue_4 (Math|Vector|MakeVector _x _y -1.5e+02) (Utilities|Array|MakeArray "ObjectTypeQuery1") false (Utilities|Array|MakeArray (Game|GetPlayerController 0)) "None"))
  (bind _asbp_player_jelly (Utilities|Casting|CastToBP_PlayerJelly (Game|Player|GetPlayerPawn 0)))
  (bind _returnvalue_5 (Rendering|Decal|SpawnDecalatLocation (Variables|Default|GetDecalMaterial) (* (Variables|Default|GetDefaultDecalSize) (Variables|/Game/GroupTings/BP/Player/BP_PlayerJelly.BP_PlayerJelly_C|GetrayCastRadius%28JellyMeshSize%29 _asbp_player_jelly)) (.Location (Collision|BreakHitResult _outhit)) "-90.000000,0.000000,0.000000" 5.0))
  (Variables|Default|SetMostRecentDecal _returnvalue_5)
  (Utilities|Array|Add (Variables|Default|GetArrayOfDecals) 0)
  (Utilities|Time|SetTimerbyEvent (delegate Custom|DecalLoop) 0.05 true))

(fn ConstructionScript)