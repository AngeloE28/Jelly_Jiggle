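; BP_RoombaNewest is a Roomba pawn with two spinning blades.
; On BeginPlay it binds a separate rotating movement component to each of the left and right blades.
; An unconnected wander chain would wait a random delay, then use AIMoveTo toward a random reachable nearby point while toggling IsMoving.
; That chain never runs, so this graph only sets up the blade rotation.
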(event EventBeginPlay
  (Components|Movement|SetUpdatedComponent (Variables|Default|GetRotatingMovementR) (Variables|Default|GetRoombaBladeR))
  (Components|Movement|SetUpdatedComponent (Variables|Default|GetRotatingMovementL) (Variables|Default|GetRoombaBladeL)))

(event Collision|EventActorBeginOverlap
  (params (OtherActor :type Actor%20Object%20Reference)))

(event EventTick
  (params (DeltaSeconds :type Float%20%28single-precision%29)))

(fn ConstructionScript)