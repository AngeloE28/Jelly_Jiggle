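; BP_RoombaNew is an AI Roomba hazard with spinning blades that sends a death message on contact and cleans up jelly trails.
; Two rotating movement components spin the left and right blades.
; DeathHitbox calls DeathMessage on BPI_Interact actors, while TrailRemover destroys overlapping JellyTrailDecal-tagged actors.
; CutsceneFixer sets EnemyAIControllerV2 as the controller class and unhides the Roomba, but its player-event binding is disconnected.
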(event OnComponentBeginOverlap(DeathHitbox)
  (params (OverlappedComponent :type Primitive%20Component%20Object%20Reference) (OtherActor :type Actor%20Object%20Reference) (OtherComp :type Primitive%20Component%20Object%20Reference) (OtherBodyIndex :type Integer) (bFromSweep :type Boolean) (SweepResult :type Hit%20Result%20Structure%20%28by%20ref%29))
  (if (Utilities|DoesObjectImplementInterface OtherActor "/Game/GroupTings/BP/Interface/BPI_Interact.BPI_Interact_C")
    (Class|BPIDeath|Death(Message) OtherActor)))

(event OnComponentBeginOverlap(TrailRemover)
  (params (OverlappedComponent :type Primitive%20Component%20Object%20Reference) (OtherActor :type Actor%20Object%20Reference) (OtherComp :type Primitive%20Component%20Object%20Reference) (OtherBodyIndex :type Integer) (bFromSweep :type Boolean) (SweepResult :type Hit%20Result%20Structure%20%28by%20ref%29))
  (if (Actor|ActorHasTag OtherActor "JellyTrailDecal")
    (Actor|DestroyActor OtherActor)))

(event Custom|CutsceneFixer
  (Variables|Default|SetAIControllerClass "/Game/GroupTings/BP/Interactable/Roomba/Test/EnemyAIControllerV2.EnemyAIControllerV2_C")
  (Rendering|SetActorHiddenInGame false))

(event EventBeginPlay
  (Components|Movement|SetUpdatedComponent (Variables|Default|GetRotatingMovementR) (Variables|Default|GetRoombaBladeR))
  (Components|Movement|SetUpdatedComponent (Variables|Default|GetRotatingMovementL) (Variables|Default|GetRoombaBladeL)))

(event Collision|EventActorBeginOverlap
  (params (OtherActor :type Actor%20Object%20Reference)))

(event EventTick
  (params (DeltaSeconds :type Float%20%28single-precision%29)))

(fn ConstructionScript)