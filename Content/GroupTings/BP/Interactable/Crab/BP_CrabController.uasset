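; AI controller for the crab enemy, running BT_Crab on possession and feeding perception results into its Blackboard.
; Sensing a player jelly cancels the forget timer and sets the Attack and EnemyActor keys.
; Lost sight, or a perception update from any other actor, starts a line-of-sight timer that clears both keys when it expires.
; KilledPlayer clears the target immediately, and FreezeBehaviour sets the Freeze key.
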(event OnTargetPerceptionUpdated(AIPerception)
  (params (Actor :type Actor%20Object%20Reference) (Stimulus :type AI%20Stimulus%20Structure))
  (bind _blackboard (Variables|Default|GetBlackboard))
  (bind _asbp_player_jelly (Utilities|Casting|CastToBP_PlayerJelly Actor)
    (:then
      (if (Utilities|Struct|BreakAIStimulus Stimulus)
        (Utilities|Time|ClearandInvalidateTimerbyHandle (Variables|Default|GetEnemyTimer))
        (AI|Components|Blackboard|SetValueasBool _blackboard (Variables|Default|GetAttack) true)
        (AI|Components|Blackboard|SetValueasObject _blackboard (Variables|Default|GetEnemyActor) _asbp_player_jelly)
        (else
          (bind _returnvalue (Utilities|Time|SetTimerbyEvent (delegate Custom|StartEnemyTimer) (Variables|Default|GetLineOfSightTimer) :!label _label))
          (Variables|Default|SetEnemyTimer _returnvalue))))
    (:CastFailed
      (goto _label))))

(event Custom|StartEnemyTimer
  (bind _blackboard (Variables|Default|GetBlackboard))
  (AI|Components|Blackboard|SetValueasBool _blackboard (Variables|Default|GetAttack) false)
  (AI|Components|Blackboard|SetValueasObject _blackboard (Variables|Default|GetEnemyActor) 0))

(event EventPossess
  (params (PossessedPawn :type Pawn%20Object%20Reference))
  (AI|RunBehaviorTree "/Game/GroupTings/BP/Interactable/Crab/BT_Crab.BT_Crab"))

(fn ConstructionScript)

(fn FreezeBehaviour
  (AI|Components|Blackboard|SetValueasBool (Variables|Default|GetBlackboard) (Variables|Default|GetFreeze) true))

(fn KilledPlayer
  (bind _blackboard (Variables|Default|GetBlackboard))
  (AI|Components|Blackboard|SetValueasBool _blackboard (Variables|Default|GetAttack) false)
  (AI|Components|Blackboard|SetValueasObject _blackboard (Variables|Default|GetEnemyActor) 0))