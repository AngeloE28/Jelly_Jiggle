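; Crab enemy character that kills the player jelly on contact and can be frozen by touching a jelly.
; Collider overlaps play the attack and death message or tell BP_CrabController to start freeze behaviour.
; Freeze stops movement, disables the death collider and spawns a BP_FreezeCrab jelly that timelines scale up, then shrink after a struggle montage.
; Unfreeze restores movement and collision, notifies the controller and destroys the jelly.
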(event OnComponentBeginOverlap(JellyCollider)
  (params (OverlappedComponent :type Primitive%20Component%20Object%20Reference) (OtherActor :type Actor%20Object%20Reference) (OtherComp :type Primitive%20Component%20Object%20Reference) (OtherBodyIndex :type Integer) (bFromSweep :type Boolean) (SweepResult :type Hit%20Result%20Structure%20%28by%20ref%29))
  (if (Utilities|ClassIsChildOf (Utilities|GetClass OtherActor) "/Game/GroupTings/BP/Interactable/Jellies/BP_JellyBase.BP_JellyBase_C")
    (bind _asbp_crab_controller (Utilities|Casting|CastToBP_CrabController (Pawn|GetController)))
    (Default|FreezeBehaviour _asbp_crab_controller)))

(event OnComponentBeginOverlap(DeathCollider)
  (params (OverlappedComponent :type Primitive%20Component%20Object%20Reference) (OtherActor :type Actor%20Object%20Reference) (OtherComp :type Primitive%20Component%20Object%20Reference) (OtherBodyIndex :type Integer) (bFromSweep :type Boolean) (SweepResult :type Hit%20Result%20Structure%20%28by%20ref%29))
  (if (Utilities|DoesObjectImplementInterface OtherActor "/Game/GroupTings/BP/Interface/BPI_Interact.BPI_Interact_C")
    (Utilities|Casting|CastToBP_PlayerJelly OtherActor)
    (Animation|Montage|PlayMontage (Variables|Character|GetMesh) "/Game/GroupTings/Characters/Crab/Animations/SM_crabAttack_Anim_Montage.SM_crabAttack_Anim_Montage"
      (:then
        (Utilities|FlowControl|RetriggerableDelay 0.2)
        (Class|BPIDeath|Death(Message) OtherActor)
        (bind _asbp_crab_controller (Utilities|Casting|CastToBP_CrabController (Pawn|GetController)))
        (Default|KilledPlayer _asbp_crab_controller)))))

(event Custom|SpawnJellyEvent
  (CallFunction|SpawnJellyAnim))

(event Custom|SpawnJellyAnim
  (bind _timetrack (Timeline|Spawn_Timeline PlayFromStart)
    (:Update
      (Transformation|SetActorScale3D (Variables|Default|GetJelly) (Math|Vector|Lerp(Vector) (Transformation|GetActorScale3D (Variables|Default|GetJelly)) "1.000000,1.000000,1.000000" _timetrack)))
    (:Finished
      (Utilities|FlowControl|RetriggerableDelay 0.7)
      (Animation|Montage|PlayMontage (Variables|Character|GetMesh) "/Game/GroupTings/Characters/Crab/Animations/SM_crabStruggle_Anim_Montage.SM_crabStruggle_Anim_Montage"
        (:then
          (CallFunction|DespawnJellyAnim))))))

(event Custom|DespawnJellyAnim
  (bind _timetrack (Timeline|Despawn_Timeline PlayFromStart)
    (:Update
      (bind _jelly (Variables|Default|GetJelly)
        (:then
          (Transformation|SetActorScale3D _jelly (Math|Vector|Lerp(Vector) (Transformation|GetActorScale3D _jelly) "0, 0, 0" _timetrack)))
        (:else)))))

(event EventBeginPlay
  (Variables|Default|SetisFrozen false)
  (EventDispatchers|BindEventtoSpawnJelly (delegate Custom|SpawnJellyEvent)))

(fn ConstructionScript)

(fn UpdateWalkSpeed
  (params (NewWalkSpeed :type Float%20%28double-precision%29))
  (Variables|/Script/Engine.CharacterMovementComponent|SetMaxWalkSpeed (Variables|Character|GetCharacterMovement) NewWalkSpeed))

(fn Freeze
  (Pawn|Components|CharacterMovement|DisableMovement (Variables|Character|GetCharacterMovement))
  (Variables|Default|SetisFrozen true)
  (Collision|SetCollisionEnabled (Variables|Default|GetDeathCollider) "NoCollision")
  (bind _returnvalue (Game|SpawnActorfromClass "/Game/GroupTings/BP/Interactable/Jellies/JellyBase_ChildClasses/BP_FreezeCrab.BP_FreezeCrab_C" (Math|Transform|MakeTransform (Transformation|GetWorldLocation (Variables|Default|GetJellySpawnLoc)) "0, 0, 0" "0.100000,0.100000,0.100000") "Undefined" 0 0))
  (bind _jelly (Variables|Default|GetJelly)
    (:then
      (Actor|DestroyActor _jelly))
    (:else
      _))
  (Variables|Default|SetJelly _returnvalue)
  (Default|CallSpawnJelly))

(fn Unfreeze
  (Pawn|Components|CharacterMovement|SetMovementMode (Variables|Character|GetCharacterMovement) "MOVE_Walking" 0)
  (Variables|Default|SetisFrozen false)
  (Collision|SetCollisionEnabled (Variables|Default|GetDeathCollider) "QueryOnly")
  (bind _asbp_crab_controller (Utilities|Casting|CastToBP_CrabController (Pawn|GetController)))
  (Default|UnfreezeBehaviour _asbp_crab_controller)
  (bind _jelly (Variables|Default|GetJelly)
    (:then
      (Actor|DestroyActor _jelly))
    (:else)))