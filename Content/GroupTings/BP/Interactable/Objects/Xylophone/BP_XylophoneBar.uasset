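; BP_XylophoneBar is a single bar of an interactable xylophone that glows and plays its sound when triggered.
; A box overlap reports the bar to its owning Xylophone, then lights it for one second.
; HintBar gives the same light and sound without reporting to the Xylophone.
; The construction script creates a dynamic material instance so each bar's emissive glow changes independently.
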(event OnComponentBeginOverlap(Box)
  (params (OverlappedComponent :type Primitive%20Component%20Object%20Reference) (OtherActor :type Actor%20Object%20Reference) (OtherComp :type Primitive%20Component%20Object%20Reference) (OtherBodyIndex :type Integer) (bFromSweep :type Boolean) (SweepResult :type Hit%20Result%20Structure%20%28by%20ref%29))
  (bind _xylophone (Variables|Default|GetXylophone)
    (:then
      (Default|CallAddBarEvent _xylophone self)
      (CallFunction|ActivateBar)
      (Utilities|FlowControl|Delay 1.0)
      (CallFunction|ResetBar))
    (:else)))

(event Custom|ResetBar
  (Rendering|Material|SetScalarParameterValue (Variables|Default|GetMaterial) (Variables|Default|GetEmissiveParameter) 0.0 :!class /Script/Engine.MaterialInstanceDynamic))

(event Custom|ActivateBar
  (Rendering|Material|SetScalarParameterValue (Variables|Default|GetMaterial) (Variables|Default|GetEmissiveParameter) 5.0 :!class /Script/Engine.MaterialInstanceDynamic)
  (Audio|PlaySoundatLocation (Variables|Default|GetSoundToPlay) (Transformation|GetWorldLocation (Variables|Default|GetBar)) "0, 0, 0" 1.0 1.0 0.0 0 0 0 0))

(event Custom|HintBar
  (CallFunction|ActivateBar)
  (Utilities|FlowControl|Delay 1.0)
  (CallFunction|ResetBar))

(fn ConstructionScript
  (bind _returnvalue (Rendering|Material|CreateDynamicMaterialInstance (Variables|Default|GetBar) 0 (Variables|Default|GetSource%20Material) "None" :!class /Script/Engine.PrimitiveComponent))
  (bind _output_get (Variables|Default|SetMaterial _returnvalue))
  (Rendering|Material|SetMaterial (Variables|Default|GetBar) 0 _output_get))