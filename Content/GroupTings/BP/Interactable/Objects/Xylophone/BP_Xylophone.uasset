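; Xylophone memory puzzle that shuffles its seven colored child bars at BeginPlay into the order the player must reproduce.
; The first Character to enter the trigger starts a timed hint sequence, after which the bars receive a reference to the xylophone.
; Reported hits are checked against the order through an event dispatcher.
; A mistake clears the references and progress, flashes all bars and replays the hint, while a full match finishes the puzzle.
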(event OnComponentBeginOverlap(EnterCollider)
  (params (OverlappedComponent :type Primitive%20Component%20Object%20Reference) (OtherActor :type Actor%20Object%20Reference) (OtherComp :type Primitive%20Component%20Object%20Reference) (OtherBodyIndex :type Integer) (bFromSweep :type Boolean) (SweepResult :type Hit%20Result%20Structure%20%28by%20ref%29))
  (Utilities|Casting|CastToCharacter OtherActor)
  (Utilities|FlowControl|DoOnce false
    (:Completed
      (CallFunction|ShowHint))))

(event Custom|GenerateOrder
  ;[1 1 1] Generate a random order
  (bind _output_get (Variables|Default|SetBarOrder (Utilities|Array|MakeArray (Variables|/Script/Engine.ChildActorComponent|GetChildActor (Variables|Default|GetBP_XylophoneBarPink)) (Variables|/Script/Engine.ChildActorComponent|GetChildActor (Variables|Default|GetBP_XylophoneBarBlue)) (Variables|/Script/Engine.ChildActorComponent|GetChildActor (Variables|Default|GetBP_XylophoneBarGreen)) (Variables|/Script/Engine.ChildActorComponent|GetChildActor (Variables|Default|GetBP_XylophoneBarYellow)) (Variables|/Script/Engine.ChildActorComponent|GetChildActor (Variables|Default|GetBP_XylophoneBarOrange)) (Variables|/Script/Engine.ChildActorComponent|GetChildActor (Variables|Default|GetBP_XylophoneBarRed)) (Variables|/Script/Engine.ChildActorComponent|GetChildActor (Variables|Default|GetBP_XylophoneBarPurple)))))
  (Utilities|Array|Shuffle _output_get))

(event Custom|AddBarToArray
  (params (ActorBar :type Actor%20Object%20Reference))
  (if (not (Variables|Default|GetPuzzleFinished))
    (Utilities|Array|Add (Variables|Default|GetHitBarOrder) ActorBar)
    (bind (_array_element _array_index) (Utilities|Array|ForEachLoopwithBreak (Variables|Default|GetHitBarOrder) :!label _label)
      (:LoopBody
        (if (== _array_element (Utilities|Array|Get(acopy) (Variables|Default|GetBarOrder) _array_index))
          (if (Utilities|Array|Identical (Variables|Default|GetHitBarOrder) (Variables|Default|GetBarOrder))
            (Variables|Default|SetPuzzleFinished true))
          (else
            (CallFunction|FailedPuzzle)
            (Utilities|FlowControl|Delay 2.0)
            (CallFunction|ShowHint)
            (goto _label Break)))))))

(event Custom|ClearXylophoneRef
  (for _array_element (Variables|Default|GetBarOrder)
    (bind _asbp_xylophone_bar (Utilities|Casting|CastToBP_XylophoneBar _array_element))
    (Variables|/Game/GroupTings/BP/Interactable/Objects/Xylophone/BP_XylophoneBar.BP_XylophoneBar_C|SetXylophone _asbp_xylophone_bar 0)))

(event Custom|AddXylophoneRef
  (for _array_element (Variables|Default|GetBarOrder)
    (bind _asbp_xylophone_bar (Utilities|Casting|CastToBP_XylophoneBar _array_element))
    (Variables|/Game/GroupTings/BP/Interactable/Objects/Xylophone/BP_XylophoneBar.BP_XylophoneBar_C|SetXylophone _asbp_xylophone_bar self)))

(event Custom|ShowHint
  (bind _arrayelement (Utilities|ForeachLoopwithDelay (Variables|Default|GetBarOrder) (Variables|Default|GetPatternDelay))
    (:LoopBody
      (bind _asbp_xylophone_bar (Utilities|Casting|CastToBP_XylophoneBar _arrayelement))
      (Default|HintBar _asbp_xylophone_bar))
    (:Complete
      (CallFunction|AddXylophoneRef))))

(event Custom|FailedPuzzle
  (CallFunction|ClearXylophoneRef)
  (Utilities|Array|Clear (Variables|Default|GetHitBarOrder))
  (for _array_element (Variables|Default|GetBarOrder)
    (bind _asbp_xylophone_bar (Utilities|Casting|CastToBP_XylophoneBar _array_element))
    (Default|ActivateBar _asbp_xylophone_bar))
  (Utilities|FlowControl|Delay 0.5)
  (for _array_element_2 (Variables|Default|GetBarOrder)
    (bind _asbp_xylophone_bar_2 (Utilities|Casting|CastToBP_XylophoneBar _array_element_2))
    (Default|ResetBar _asbp_xylophone_bar_2)))

(event EventBeginPlay
  (CallFunction|GenerateOrder)
  (EventDispatchers|BindEventtoAddBarEvent (delegate Custom|AddBarToArray)))

(fn ConstructionScript)