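; BP_Hat is an interactable hat that trails the jelly player while the jelly is small.
; Interacting toggles following, allowed only when the player's capsule X scale is below JellyMinSize.
; While following, Tick zeroes the hat's rotation and teleports it along an interpolated XY path toward the player beyond MinDistanceToPlayer, keeping its Z.
; Following stops when the jelly exceeds that size or any Character leaves LeaveCollider.
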(event OnComponentEndOverlap(LeaveCollider)
  (params (OverlappedComponent :type Primitive%20Component%20Object%20Reference) (OtherActor :type Actor%20Object%20Reference) (OtherComp :type Primitive%20Component%20Object%20Reference) (OtherBodyIndex :type Integer))
  (Utilities|Casting|CastToCharacter OtherActor)
  (Variables|Default|SetInteracted false))

(event EventTick
  (params (DeltaSeconds :type Float%20%28single-precision%29))
  (bind _returnvalue (Utilities|Time|GetWorldDeltaSeconds))
  (bind _hat (Variables|Default|GetHat))
  (bind _interactor (Variables|Default|GetInteractor))
  (bind _returnvalue_2 (Transformation|GetActorLocation _interactor))
  (bind _returnvalue_3 (Transformation|GetWorldLocation _hat))
  (bind _returnvalue_4 (Math|Vector2D|MakeVector2D (.x _returnvalue_2) (.y _returnvalue_2)))
  (bind _returnvalue_5 (Math|Vector2D|MakeVector2D (.x _returnvalue_3) (.y _returnvalue_3)))
  (bind _returnvalue_6 (Class|KismetMathLibrary|Vector2DInterpto _returnvalue_5 _returnvalue_4 _returnvalue 1e+01))
  (if (Variables|Default|GetInteracted)
    (Utilities|FlowControl|Sequence
      (:then_0
        (Transformation|SetWorldRotation (Variables|Default|GetHat) (Math|Rotator|MakeRotator 0.0 0.0 0.0) false false)
        (if (>= (Math|Vector|Distance2D(Vector) _returnvalue_5 _returnvalue_4) (Variables|Default|GetMinDistanceToPlayer))
          (Transformation|SetWorldLocation _hat (Math|Vector|MakeVector (.x _returnvalue_6) (.y _returnvalue_6) (.z _returnvalue_3)) false true)))
      (:then_1
        (if (> (.x (Transformation|GetWorldScale (Variables|/Script/Engine.Character|GetCapsuleComponent (Variables|Default|GetInteractor)))) (Variables|Default|GetJellyMinSize))
          (Variables|Default|SetInteracted false))))))

(event EventInteractbyInteracting
  (params (Interactor :type Character%20Object%20Reference))
  (bind _asbp_player_jelly (Utilities|Casting|CastToBP_PlayerJelly Interactor))
  (bind _output_get (Variables|Default|SetInteractor _asbp_player_jelly))
  (if (< (.x (Transformation|GetWorldScale (Variables|/Script/Engine.Character|GetCapsuleComponent _output_get))) (Variables|Default|GetJellyMinSize))
    (if (Variables|Default|GetInteracted)
      (Variables|Default|SetInteracted false)
      (else
        (Variables|Default|SetInteracted true)))
    (else
      (Variables|Default|SetInteracted false))))

(fn ConstructionScript)