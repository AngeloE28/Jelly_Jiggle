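; BP_LevelEnd is the level exit trigger that advances the player through the Kitchen, Backyard, Sewer and Beach sequence.
; When either player jelly blueprint overlaps it, it checks the current level name, then sets the next scene on BP_LoadingGameInstance and starts the loading screen fade-in.
; On Beach, the last level, it instead shows the level complete widget with mouse cursor and UI-only input, and disables player movement.
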(event Collision|EventActorBeginOverlap
  (params (OtherActor :type Actor%20Object%20Reference))
  (bind _returnvalue (Game|GetPlayerController 0))
  (Utilities|Casting|CastToBP_PlayerJelly OtherActor
    (:then
      _)
    (:CastFailed
      (Utilities|Casting|CastToBP_PlayerJellySewerV3 OtherActor)))
  (bind _returnvalue_2 (Game|GetCurrentLevelName true))
  (if (Utilities|Enum|Equal(Enum) _returnvalue_2 "Kitchen")
    (bind _asbp_loading_game_instance (Utilities|Casting|CastToBP_LoadingGameInstance (Game|GetGameInstance)))
    (Variables|/Game/GroupTings/BP/LevelLoading/BP_LoadingGameInstance.BP_LoadingGameInstance_C|SetsceneToLoad _asbp_loading_game_instance "/Game/GroupTings/Levels/Backyard.Backyard")
    (Default|LoadingScreenFadein _asbp_loading_game_instance)
    (elif (Utilities|Enum|Equal(Enum) _returnvalue_2 "Backyard")
      (bind _asbp_loading_game_instance_2 (Utilities|Casting|CastToBP_LoadingGameInstance (Game|GetGameInstance)))
      (Variables|/Game/GroupTings/BP/LevelLoading/BP_LoadingGameInstance.BP_LoadingGameInstance_C|SetsceneToLoad _asbp_loading_game_instance_2 "/Game/GroupTings/Levels/Sewer.Sewer")
      (Default|LoadingScreenFadein _asbp_loading_game_instance_2)
      (elif (Utilities|Enum|Equal(Enum) _returnvalue_2 "Sewer")
        (bind _asbp_loading_game_instance_3 (Utilities|Casting|CastToBP_LoadingGameInstance (Game|GetGameInstance)))
        (Variables|/Game/GroupTings/BP/LevelLoading/BP_LoadingGameInstance.BP_LoadingGameInstance_C|SetsceneToLoad _asbp_loading_game_instance_3 "/Game/GroupTings/Levels/Beach.Beach")
        (Default|LoadingScreenFadein _asbp_loading_game_instance_3)
        (elif (Utilities|Enum|Equal(Enum) _returnvalue_2 "Beach")
          (bind _returnvalue_3 (UserInterface|CreateWidget "/Game/GroupTings/BP/UI/WBP_LevelComplete.WBP_LevelComplete_C"))
          (UserInterface|Viewport|AddtoViewport _returnvalue_3 0)
          (Variables|/Script/Engine.PlayerController|SetbShowMouseCursor _returnvalue true)
          (Input|SetInputModeUIOnly _returnvalue _returnvalue_3 "DoNotLock")
          (Pawn|Components|CharacterMovement|DisableMovement (Variables|/Script/Engine.Character|GetCharacterMovement (Game|GetPlayerCharacter 0))))))))

(fn ConstructionScript)