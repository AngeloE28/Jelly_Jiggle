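; Checkpoint actor that moves the respawn point when the jelly player (BP_PlayerJelly) enters its Collider.
; On overlap it asks BP_ThirdPersonGameMode for player 0's current PlayerStart and destroys it if one exists.
; It then spawns a new PlayerStart at the world location and rotation of its SpawnLocation component.
; Nothing marks the checkpoint as used, so every re-entry repeats the swap.
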(event OnComponentBeginOverlap(Collider)
  (params (OverlappedComponent :type Primitive%20Component%20Object%20Reference) (OtherActor :type Actor%20Object%20Reference) (OtherComp :type Primitive%20Component%20Object%20Reference) (OtherBodyIndex :type Integer) (bFromSweep :type Boolean) (SweepResult :type Hit%20Result%20Structure%20%28by%20ref%29))
  (bind _spawnlocation (Variables|Default|GetSpawnLocation))
  (bind _spawnlocation_2 (Variables|Default|GetSpawnLocation))
  (Utilities|Casting|CastToBP_PlayerJelly OtherActor)
  (bind _asbp_third_person_game_mode (Utilities|Casting|CastToBP_ThirdPersonGameMode (Game|GetGameMode)))
  (Utilities|IsValid (Class|GameModeBase|FindPlayerStart _asbp_third_person_game_mode (Game|GetPlayerController 0))
    (:Is%20Valid
      (Actor|DestroyActor (Class|GameModeBase|FindPlayerStart _asbp_third_person_game_mode (Game|GetPlayerController 0)))
      (Game|SpawnActorfromClass "/Script/Engine.PlayerStart" (Math|Transform|MakeTransform (Transformation|GetWorldLocation _spawnlocation_2) (Transformation|GetWorldRotation _spawnlocation_2) "1.000000,1.000000,1.000000") "Undefined" 0 0))
    (:Is%20Not%20Valid
      (Game|SpawnActorfromClass "/Script/Engine.PlayerStart" (Math|Transform|MakeTransform (Transformation|GetWorldLocation _spawnlocation) (Transformation|GetWorldRotation _spawnlocation) "1.000000,1.000000,1.000000") "Undefined" 0 0))))

(fn ConstructionScript)