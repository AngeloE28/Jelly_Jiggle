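; An example jelly pickup Blueprint that grants the interacting player a temporary double jump.
; InteractWithPlayer raises the Character's JumpMaxCount to 2, then calls the parent's shared HideToDestroyLater to remove the pickup.
; FinishTimedUpgrade sets the jump count back to 1, while GetInteractionValues reports whether the power is time-limited and for how long.
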(fn ConstructionScript
  (|CallParentFunction))

(fn InteractwithPlayer
  (params (Player :type Actor%20Object%20Reference))
  (Utilities|IsValid Player
    (:Is%20Valid
      (bind _ascharacter (Utilities|Casting|CastToCharacter Player))
      (Variables|/Script/Engine.Character|SetJumpMaxCount _ascharacter 2)
      ;[1 0 0.03843] Parent function since most child objects will use it to stop repeating using the same nodes
      (CallFunction|HidetoDestroyLater)
      (return))))

(fn FinishTimedUpgrade
  (params (Actor :type Actor%20Object%20Reference))
  (Utilities|IsValid Actor
    (:Is%20Valid
      (bind _ascharacter (Utilities|Casting|CastToCharacter Actor))
      (Variables|/Script/Engine.Character|SetJumpMaxCount _ascharacter 1)
      (return))))

(fn GetInteractionValues
  (return (Variables|Default|GethasTimeLimit) (Variables|Default|GetPowerTimeLimit)))