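; BP_JellyExampleSpeedUp is an example child of the jelly interactable base that gives the interacting character a timed speed boost.
; On interaction it doubles the character's MaxWalkSpeed and calls the parent's HideToDestroyLater.
; FinishTimedUpgrade halves the speed again to undo the boost.
; GetInteractionValues reports the time-limit flag, destroy flag and power duration to the caller.
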(fn ConstructionScript
  (|CallParentFunction))

(fn InteractwithPlayer
  (params (Player :type Actor%20Object%20Reference))
  (Utilities|IsValid Player
    (:Is%20Valid
      (bind _ascharacter (Utilities|Casting|CastToCharacter Player))
      (Variables|/Script/Engine.CharacterMovementComponent|SetMaxWalkSpeed (Variables|/Script/Engine.Character|GetCharacterMovement _ascharacter) (* (Variables|/Script/Engine.CharacterMovementComponent|GetMaxWalkSpeed (Variables|/Script/Engine.Character|GetCharacterMovement _ascharacter)) 2.0))
      ;[1 0 0.03843] Parent function since most child objects will use it to stop repeating using the same nodes
      (CallFunction|HidetoDestroyLater)
      (return))))

(fn FinishTimedUpgrade
  (params (Actor :type Actor%20Object%20Reference))
  (Utilities|IsValid Actor
    (:Is%20Valid
      (bind _ascharacter (Utilities|Casting|CastToCharacter Actor))
      (Variables|/Script/Engine.CharacterMovementComponent|SetMaxWalkSpeed (Variables|/Script/Engine.Character|GetCharacterMovement _ascharacter) (* (Variables|/Script/Engine.CharacterMovementComponent|GetMaxWalkSpeed (Variables|/Script/Engine.Character|GetCharacterMovement _ascharacter)) 0.5))
      (return))))

(fn GetInteractionValues
  (return (Variables|Default|GethasTimeLimit) (Variables|Default|GetshouldDestroy) (Variables|Default|GetpowerTimeLimit)))