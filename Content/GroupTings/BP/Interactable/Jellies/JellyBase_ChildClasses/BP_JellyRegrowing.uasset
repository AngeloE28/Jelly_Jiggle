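; Regrowing jelly pickup that a character absorbs on touch and that grows back once they leave.
; Box begin overlap drops the mesh, calls RespawnJellyGrowth on the player's BP_PlayerJelly and clears Absorbable.
; Box end overlap waits briefly, then runs Niagara while the Movement timeline lerps the mesh back up and re-arms Absorbable.
; End overlap does not check Absorbable, so any character leaving triggers the regrow.
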(event OnComponentBeginOverlap(Box)
  (params (OverlappedComponent :type Primitive%20Component%20Object%20Reference) (OtherActor :type Actor%20Object%20Reference) (OtherComp :type Primitive%20Component%20Object%20Reference) (OtherBodyIndex :type Integer) (bFromSweep :type Boolean) (SweepResult :type Hit%20Result%20Structure%20%28by%20ref%29))
  (if (Variables|Default|GetAbsorbable?)
    (if (Utilities|ClassIsChildOf (Utilities|GetClass OtherActor) "/Script/Engine.Character")
      (Transformation|SetRelativeLocation (Variables|Default|GetStaticMesh) (+ (Variables|/Script/Engine.SceneComponent|GetRelativeLocation (Variables|Default|GetStaticMesh)) "0,0,-40.000000") false true)
      (bind _asbp_player_jelly (Utilities|Casting|CastToBP_PlayerJelly (Game|Player|GetPlayerPawn 0)))
      (Default|RespawnJellyGrowth _asbp_player_jelly)
      (Variables|Default|SetAbsorbable? false))))

(event OnComponentEndOverlap(Box)
  (params (OverlappedComponent :type Primitive%20Component%20Object%20Reference) (OtherActor :type Actor%20Object%20Reference) (OtherComp :type Primitive%20Component%20Object%20Reference) (OtherBodyIndex :type Integer))
  (if (Utilities|ClassIsChildOf (Utilities|GetClass OtherActor) "/Script/Engine.Character")
    (Utilities|FlowControl|Delay 3.0)
    (Components|Activation|Activate (Variables|Default|GetNiagara) false)
    (bind _alpha (Timeline|Movement PlayFromStart)
      (:Update
        (Transformation|SetRelativeLocation (Variables|Default|GetStaticMesh) (Math|Vector|Lerp(Vector) "0, 0,-40.000000" "0, 0,0.000000" _alpha) false false))
      (:Finished
        (Variables|Default|SetAbsorbable? true)
        (Components|Activation|Deactivate (Variables|Default|GetNiagara))))))

(event EventBeginPlay)

(event Collision|EventActorBeginOverlap
  (params (OtherActor :type Actor%20Object%20Reference)))

(event EventTick
  (params (DeltaSeconds :type Float%20%28single-precision%29)))

(fn ConstructionScript)