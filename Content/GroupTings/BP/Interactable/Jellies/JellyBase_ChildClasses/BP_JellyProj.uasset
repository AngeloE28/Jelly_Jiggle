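; BP_JellyProj is a jelly projectile that splats on impact and becomes an interactable BP_JellyGrow when it stops moving.
; The construction script applies JellySpeed to ProjectileMovement, whose updated component is switched to the sphere collider on activation.
; Each hit plays splat sound and particles, spawns a trail decal, and pushes physics-simulating objects using velocity and ImpulseForce.
; On stop, it spawns the replacement at the mesh transform, removes the latest decal and destroys itself.
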(event OnComponentActivated(ProjectileMovement)
  (params (Component :type Actor%20Component%20Object%20Reference) (bReset :type Boolean))
  ;[1 1 1] Updated component should be the sphere collider instead of root component
  (Components|Movement|SetUpdatedComponent (Variables|Default|GetProjectileMovement) (Variables|Default|GetProjectileCollider)))

(event OnProjectileStop(ProjectileMovement)
  (params (ImpactResult :type Hit%20Result%20Structure%20%28by%20ref%29))
  ;[1 1 1] Replace projectile with an interactable jelly when the projectile is not moving anymore
  (Components|Activation|Deactivate (Variables|Default|GetProjectileMovement))
  (Game|SpawnActorfromClass "/Game/GroupTings/BP/Interactable/Jellies/JellyBase_ChildClasses/BP_JellyGrow.BP_JellyGrow_C" (Transformation|GetWorldTransform (Variables|Default|GetMesh)) "Undefined" 0 0)
  (Components|DestroyComponent (stale Collision|EventHit _returnvalue_2))
  (Actor|DestroyActor))

(event EventBeginPlay)

(event Collision|EventHit
  (params (MyComp :type Primitive%20Component%20Object%20Reference) (Other :type Actor%20Object%20Reference) (OtherComp :type Primitive%20Component%20Object%20Reference) (bSelfMoved :type Boolean) (HitLocation :type Vector :default "0, 0, 0") (HitNormal :type Vector :default "0, 0, 0") (NormalImpulse :type Vector :default "0, 0, 0") (Hit :type Hit%20Result%20Structure%20%28by%20ref%29))
  (bind _projectilecollider (Variables|Default|GetProjectileCollider))
  (bind _impulseforce (Variables|Default|GetimpulseForce))
  (bind _returnvalue (Transformation|GetWorldLocation _projectilecollider))
  (Audio|PlaySoundatLocation "/Game/GroupTings/SFX/Player/Splat/SC_Splat.SC_Splat" _returnvalue "0, 0, 0" 0.2 1.0 0.0 0 "/Game/GroupTings/SFX/SCC_JellyProj.SCC_JellyProj" 0 0)
  (Niagara|SpawnSystematLocation "/Game/GroupTings/FX/tut/P_Splash.P_Splash" _returnvalue)
  (bind _returnvalue_2 (Rendering|Decal|SpawnDecalatLocation "/Game/GroupTings/FX/JellyTrailNew/Mat_Jelly_TrailV2.Mat_Jelly_TrailV2" "80.000000,80.000000,80.000000" _returnvalue "-90.000000,0.000000,0.000000" 5.0))
  ;[1 1 1] Add Impulse on Collision
  (if (Physics|IsSimulatingPhysics OtherComp "None")
    (Physics|AddImpulseatLocation OtherComp (* (* (Variables|/Script/Engine.MovementComponent|GetVelocity (Variables|Default|GetProjectileMovement)) _impulseforce) (/ _impulseforce 4.0)) (Transformation|GetActorLocation) "None")))

(fn ConstructionScript
  (bind _projectilemovement (Variables|Default|GetProjectileMovement))
  (Variables|/Script/Engine.ProjectileMovementComponent|SetMaxSpeed _projectilemovement (Variables|Default|GetJellySpeed))
  (Variables|/Script/Engine.ProjectileMovementComponent|SetInitialSpeed _projectilemovement (Variables|Default|GetJellySpeed)))