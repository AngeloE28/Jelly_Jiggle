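; BP_JellyJump is a jelly interactable that carries the player along a spline and launches them off it.
; On interaction it applies the player's stronger falling gravity, then a timeline scaled by air time moves the capsule and rotates the mesh along the spline.
; Past a set point on the path, it launches the character along the spline tangent.
; Collider overlaps drive a jiggle timeline that writes impact position and normal to a Material Parameter Collection.
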(event OnComponentEndOverlap(JellyCollider)
  (params (OverlappedComponent :type Primitive%20Component%20Object%20Reference) (OtherActor :type Actor%20Object%20Reference) (OtherComp :type Primitive%20Component%20Object%20Reference) (OtherBodyIndex :type Integer))
  (Variables|Default|SetImpact%20Normal (.ImpactNormal (Collision|BreakHitResult (stale OnComponentBeginOverlap(JellyCollider) SweepResult))))
  (Rendering|Material|SetVectorParameterValue "/Game/GroupTings/Materials/Jiggle/Data/MPC_JiggleData.MPC_JiggleData" "Position" (Math|Conversions|ToLinearColor(Vector) (.ImpactPoint (Collision|BreakHitResult (stale OnComponentBeginOverlap(JellyCollider) SweepResult)))) :!class /Script/Engine.KismetMaterialLibrary)
  (bind _jiggle_track (Timeline|Jiggle_Timeline PlayFromStart)
    (:Update
      (Rendering|Material|SetVectorParameterValue "/Game/GroupTings/Materials/Jiggle/Data/MPC_JiggleData.MPC_JiggleData" "Normal" (Math|Conversions|ToLinearColor(Vector) (* (Variables|Default|GetImpact%20Normal) (* _jiggle_track (Variables|Default|GetjiggleStrength)))) :!class /Script/Engine.KismetMaterialLibrary))))

(event OnComponentBeginOverlap(JellyCollider)
  (params (OverlappedComponent :type Primitive%20Component%20Object%20Reference) (OtherActor :type Actor%20Object%20Reference) (OtherComp :type Primitive%20Component%20Object%20Reference) (OtherBodyIndex :type Integer) (bFromSweep :type Boolean) (SweepResult :type Hit%20Result%20Structure%20%28by%20ref%29))
  (bind (_bblockinghit _binitialoverlap _time _distance _location _impactpoint _normal _impactnormal) (Collision|BreakHitResult SweepResult))
  (Variables|Default|SetImpact%20Normal _impactnormal)
  (Rendering|Material|SetVectorParameterValue "/Game/GroupTings/Materials/Jiggle/Data/MPC_JiggleData.MPC_JiggleData" "Position" (Math|Conversions|ToLinearColor(Vector) _impactpoint) :!class /Script/Engine.KismetMaterialLibrary)
  (bind _jiggle_track (Timeline|Jiggle_Timeline PlayFromStart)
    (:Update
      (Rendering|Material|SetVectorParameterValue "/Game/GroupTings/Materials/Jiggle/Data/MPC_JiggleData.MPC_JiggleData" "Normal" (Math|Conversions|ToLinearColor(Vector) (* (Variables|Default|GetImpact%20Normal) (* _jiggle_track (Variables|Default|GetjiggleStrength)))) :!class /Script/Engine.KismetMaterialLibrary))))

(event Custom|MoveAlongPath
  (params (Player :type BP%20Player%20Jelly%20Object%20Reference))
  (bind _capsulecomponent (Variables|/Script/Engine.Character|GetCapsuleComponent Player))
  (bind _returnvalue (Transformation|GetWorldTransform _capsulecomponent))
  (Components|Timeline|SetPlayRate (Variables|Default|GetMove_Timeline) (/ 1.0 (Variables|Default|GetPlayerAirTime)))
  (bind _movetrack (Timeline|Move_Timeline PlayFromStart)
    (:Update
      (Transformation|SetWorldTransform _capsulecomponent (Math|Transform|MakeTransform (Spline|GetLocationatDistanceAlongSpline (Variables|Default|GetSpline) (Math|Float|Lerp 0.0 (Spline|GetSplineLength (Variables|Default|GetSpline)) _movetrack) "World") (.rotation _returnvalue) (.scale _returnvalue)) false false)
      (Transformation|SetWorldRotation (Variables|/Script/Engine.Character|GetMesh Player) (Spline|GetRotationatDistanceAlongSpline (Variables|Default|GetSpline) (Math|Float|Lerp 0.0 (Spline|GetSplineLength (Variables|Default|GetSpline)) _movetrack) "World") false false)
      (if (> _movetrack (Variables|Default|GetMaxDistAlongSplinePath))
        (Utilities|FlowControl|DoOnce false :!label _label
          (:Completed
            (Character|LaunchCharacter Player (* (Math|Vector|Normalize (Math|Rotator|GetRotationXVector (Spline|GetRotationatDistanceAlongSpline (Variables|Default|GetSpline) (Math|Float|Lerp 0.0 (Spline|GetSplineLength (Variables|Default|GetSpline)) _movetrack) "World"))) (Variables|Default|GetlaunchStrength)) true false)
            (Timeline|Move_Timeline Stop)))))
    (:Finished
      (goto _label Reset))))

(fn ConstructionScript
  (|CallParentFunction))

(fn InteractwithPlayer
  (params (Player :type Actor%20Object%20Reference))
  (Utilities|IsValid Player
    (:Is%20Valid
      (bind _asbp_player_jelly (Utilities|Casting|CastToBP_PlayerJelly Player))
      (Variables|/Script/Engine.CharacterMovementComponent|SetGravityScale (Variables|/Script/Engine.Character|GetCharacterMovement _asbp_player_jelly) (Variables|/Game/GroupTings/BP/Player/BP_PlayerJelly.BP_PlayerJelly_C|GetstrongerGravityScaleFalling _asbp_player_jelly))
      (CallFunction|MoveAlongPath _asbp_player_jelly))))

(fn FinishTimedUpgrade
  (params (Actor :type Actor%20Object%20Reference))
  (Utilities|IsValid Actor
    (:Is%20Valid
      (Utilities|Casting|CastToBP_PlayerJelly Actor))))