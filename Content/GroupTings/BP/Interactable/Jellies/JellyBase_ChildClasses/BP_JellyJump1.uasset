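; BP_JellyJump1 is a jelly interactable that bounces characters away and jiggles on contact.
; Collider overlap stores the impact normal and writes the impact point to the MPC_JiggleData material parameter collection.
; A timeline restarts on each overlap, driving the collection's Normal vector from that normal, the jiggle track and JiggleStrength.
; InteractWithPlayer launches the character along the stored normal at LaunchStrength, overriding its current velocity.
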(event OnComponentBeginOverlap(JellyCollider)
  (params (OverlappedComponent :type Primitive%20Component%20Object%20Reference) (OtherActor :type Actor%20Object%20Reference) (OtherComp :type Primitive%20Component%20Object%20Reference) (OtherBodyIndex :type Integer) (bFromSweep :type Boolean) (SweepResult :type Hit%20Result%20Structure%20%28by%20ref%29))
  (bind (_bblockinghit _binitialoverlap _time _distance _location _impactpoint _normal _impactnormal) (Collision|BreakHitResult SweepResult))
  (Variables|Default|SetImpact%20Normal _impactnormal)
  (Rendering|Material|SetVectorParameterValue "/Game/GroupTings/Materials/Jiggle/Data/MPC_JiggleData.MPC_JiggleData" "Position" (Math|Conversions|ToLinearColor(Vector) _impactpoint) :!class /Script/Engine.KismetMaterialLibrary)
  (bind _jiggle_track (Timeline|Jiggle_Timeline PlayFromStart)
    (:Update
      (Rendering|Material|SetVectorParameterValue "/Game/GroupTings/Materials/Jiggle/Data/MPC_JiggleData.MPC_JiggleData" "Normal" (Math|Conversions|ToLinearColor(Vector) (* (Variables|Default|GetImpact%20Normal) (* _jiggle_track (Variables|Default|GetjiggleStrength)))) :!class /Script/Engine.KismetMaterialLibrary))))

(fn ConstructionScript
  (|CallParentFunction))

(fn InteractwithPlayer
  (params (Player :type Actor%20Object%20Reference))
  (Utilities|IsValid Player
    (:Is%20Valid
      (bind _ascharacter (Utilities|Casting|CastToCharacter Player))
      (Character|LaunchCharacter _ascharacter (* (Math|Vector|Normalize (Variables|Default|GetImpact%20Normal)) (Variables|Default|GetlaunchStrength)) true true))))