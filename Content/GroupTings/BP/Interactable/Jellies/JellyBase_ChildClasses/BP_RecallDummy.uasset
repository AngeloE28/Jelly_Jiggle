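; BP_RecallDummy is a short-lived jelly actor that plays a recall visual effect, then destroys itself after a brief delay.
; On BeginPlay it spawns the N_Recall_System effect, and each Tick it rotates and moves that effect to its own location.
; It also binds to the game mode's player-death event, which runs a timeline that shrinks the jelly mesh to zero before destroying the actor.
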(event Custom|PlayerDied
  (params (Character :type Character%20Object%20Reference))
  (bind _deathtrack (Timeline|Death_Timeline PlayFromStart)
    (:Update
      (Transformation|SetWorldScale3D (Variables|Default|GetJelly) (Math|Vector|Lerp(Vector) (Transformation|GetActorScale3D) "0, 0, 0" _deathtrack)))
    (:Finished
      (Actor|DestroyActor))))

(event EventTick
  (params (DeltaSeconds :type Float%20%28single-precision%29))
  (Class|Actor|AddActorWorldRotation (Math|Conversions|RotationFromXVector (+ (Transformation|GetActorRotation) (* (Transformation|GetActorForwardVector) (Variables|Default|GetRotationSpeed) (Utilities|Time|GetWorldDeltaSeconds)))))
  (Transformation|SetWorldLocation (Variables|Default|GetTrailFX) (Transformation|GetActorLocation) false false))

(event EventBeginPlay
  (bind _returnvalue (Transformation|GetActorTransform))
  (bind _returnvalue_2 (Niagara|SpawnSystematLocation "/Game/GroupTings/FX/RecallTrail/N_Recall_System.N_Recall_System" (.location _returnvalue) (.rotation _returnvalue) (.scale _returnvalue)))
  (Variables|Default|SetTrailFX _returnvalue_2)
  (bind _asbp_third_person_game_mode (Utilities|Casting|CastToBP_ThirdPersonGameMode (Game|GetGameMode)))
  (EventDispatchers|BindEventtoOnPlayerDied _asbp_third_person_game_mode (delegate Custom|PlayerDied))
  (Utilities|FlowControl|Delay 1.2)
  (Utilities|IsValid self
    (:Is%20Valid
      (Actor|DestroyActor))))

(fn ConstructionScript)