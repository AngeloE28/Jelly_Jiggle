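; BP_JellyProj is a jelly projectile that turns into an interactable BP_JellyGrow jelly where it comes to rest.
; The construction script sets its speed from JellySpeed, and on activation the movement component drives the sphere collider instead of the root.
; Hits push physics-simulating components with a velocity-based impulse.
; When movement stops, it spawns the jelly at the mesh's transform and destroys itself.
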(event OnComponentActivated(ProjectileMovement)
  (params (Component :type Actor%20Component%20Object%20Reference) (bReset :type Boolean))
  ;[1 1 1] Updated component should be the sphere collider instead of root component
  (Components|Movement|SetUpdatedComponent (Variables|Default|GetProjectileMovement) (Variables|Default|GetProjectileCollider)))

(event OnProjectileStop(ProjectileMovement)
  (params (ImpactResult :type Hit%20Result%20Structure%20%28by%20ref%29))
  ;[1 1 1] Replace projectile with an interactable jelly when the projectile is not moving anymore
  (Components|Activation|Deactivate (Variables|Default|GetProjectileMovement))
  (Game|SpawnActorfromClass "/Game/GroupTings/BP/Interactable/Jellies/BP_JellyGrow.BP_JellyGrow_C" (Transformation|GetWorldTransform (Variables|Default|GetMesh)) "Undefined" 0 0)
  (Actor|DestroyActor))

(event EventBeginPlay)

(event Collision|EventHit
  (params (MyComp :type Primitive%20Component%20Object%20Reference) (Other :type Actor%20Object%20Reference) (OtherComp :type Primitive%20Component%20Object%20Reference) (bSelfMoved :type Boolean) (HitLocation :type Vector :default "0, 0, 0") (HitNormal :type Vector :default "0, 0, 0") (NormalImpulse :type Vector :default "0, 0, 0") (Hit :type Hit%20Result%20Structure%20%28by%20ref%29))
  (bind _impulseforce (Variables|Default|GetimpulseForce))
  ;[1 1 1] Add Impulse on Collision
  (if (Physics|IsSimulatingPhysics OtherComp "None")
    (Physics|AddImpulseatLocation OtherComp (* (* (Variables|/Script/Engine.MovementComponent|GetVelocity (Variables|Default|GetProjectileMovement)) _impulseforce) (/ _impulseforce 4.0)) (Transformation|GetActorLocation) "None")))

(fn ConstructionScript
  (bind _projectilemovement (Variables|Default|GetProjectileMovement))
  (Variables|/Script/Engine.ProjectileMovementComponent|SetMaxSpeed _projectilemovement (Variables|Default|GetJellySpeed))
  (Variables|/Script/Engine.ProjectileMovementComponent|SetInitialSpeed _projectilemovement (Variables|Default|GetJellySpeed)))