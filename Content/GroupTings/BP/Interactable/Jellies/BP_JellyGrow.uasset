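; BP_JellyGrow is a jelly interactable that shows a waypoint marker, labeled as the jelly widget, while a character is nearby.
; Actor begin and end overlap events check that the other actor is a Character, then show or hide the Waypoint component.
; The end event hides it even if another character still overlaps.
; The graph holds no grow logic, and the construction script is empty.
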(event Collision|EventActorBeginOverlap
  (params (OtherActor :type Actor%20Object%20Reference))
  ;[1 1 1] Jelly Widget
  (if (Utilities|ClassIsChildOf (Utilities|GetClass OtherActor) "/Script/Engine.Character")
    (Rendering|SetVisibility (Variables|Default|GetWaypoint) true false)))

(event Collision|EventActorEndOverlap
  (params (OtherActor :type Actor%20Object%20Reference))
  ;[1 1 1] Jelly Widget
  (if (Utilities|ClassIsChildOf (Utilities|GetClass OtherActor) "/Script/Engine.Character")
    (Rendering|SetVisibility (Variables|Default|GetWaypoint) false false)))

(fn ConstructionScript)