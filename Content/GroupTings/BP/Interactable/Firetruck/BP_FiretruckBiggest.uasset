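; Drivable firetruck vehicle with an orbit camera and a raisable ladder.
; Interacting hides the interactor and possesses the truck; pressing Interact again places that actor at the truck's mesh and returns control.
; Axis inputs drive steering, throttle, brake and spring arm, while holding Up or Down plays or reverses the ladder rotation timeline.
; Tick shows a reset widget once when roll or pitch exceeds a tipping threshold; Reset lifts and rights the truck.
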(event EventInteractbyInteracting
  (params (Interactor :type Character%20Object%20Reference))
  (Rendering|SetActorHiddenInGame Interactor true)
  (Collision|SetActorEnableCollision Interactor false)
  (Pawn|Possess (Game|GetPlayerController 0) self))

(event EventTick
  (params (DeltaSeconds :type Float%20%28single-precision%29))
  (bind _returnvalue (Transformation|GetActorRotation))
  (if (or (> (.roll _returnvalue) 85.0) (> (.pitch _returnvalue) 85.0))
    (Utilities|FlowControl|DoOnce false
      (:Completed
        (bind _returnvalue_2 (UserInterface|CreateWidget "/Game/GroupTings/BP/UI/WBP_Reset.WBP_Reset_C"))
        (bind _output_get (Variables|Default|SetResetUI _returnvalue_2))
        (UserInterface|Viewport|AddtoViewport _output_get 0)))))

(event Input|ActionEvents|InputActionInteract
  (params (Key :type Key%20Structure :default "None"))
  (bind _skeletalmesh (Variables|Default|GetSkeletalMesh))
  (:Pressed
    (Transformation|SetActorLocation (stale EventInteractbyInteracting Interactor) (Transformation|GetWorldLocation _skeletalmesh) false true)
    (Transformation|SetActorRotation (stale EventInteractbyInteracting Interactor) (Transformation|GetWorldRotation _skeletalmesh) true)
    (Rendering|SetActorHiddenInGame (stale EventInteractbyInteracting Interactor) false)
    (Collision|SetActorEnableCollision (stale EventInteractbyInteracting Interactor) true)
    (Pawn|Possess (Game|GetPlayerController 0) (stale EventInteractbyInteracting Interactor))))

(event Input|ActionEvents|InputActionUp
  (params (Key :type Key%20Structure :default "None"))
  (:Pressed
    (bind _laddermove (Timeline|Timeline_0 Play)
      (:Update
        (Transformation|SetRelativeRotation (Variables|Default|GetLadder) (Math|Rotator|Lerp(Rotator) "0,-90.000000, 0" "0,-90.000000,-30.000000" _laddermove) false false))))
  (:Released
    (Timeline|Timeline_0 Stop)))

(event Input|ActionEvents|InputActionDown
  (params (Key :type Key%20Structure :default "None"))
  (:Pressed
    (bind _laddermove (Timeline|Timeline_0 Reverse)
      (:Update
        (Transformation|SetRelativeRotation (Variables|Default|GetLadder) (Math|Rotator|Lerp(Rotator) "0,-90.000000, 0" "0,-90.000000,-30.000000" _laddermove) false false))))
  (:Released
    (Timeline|Timeline_0 Stop)))

(event Input|ActionEvents|InputActionReset
  (params (Key :type Key%20Structure :default "None"))
  (:Pressed
    (Transformation|Teleport (+ (Transformation|GetActorLocation) "0,0,150.000000") (Math|Rotator|MakeRotator 0.0 0.0 (.yaw (Transformation|GetActorRotation))))
    (bind _resetui (Variables|Default|GetResetUI)
      (:then
        (Widget|RemovefromParent _resetui)
        (Utilities|FlowControl|DoOnce false) ; enters at Reset
      )
      (:else
        (Utilities|FlowControl|DoOnce false) ; enters at Reset
      ))))

(event Input|AxisEvents|InputAxisThrottle
  (params (AxisValue :type Float%20%28single-precision%29))
  (bind _vehiclemovementcomponent (Variables|Default|GetVehicleMovementComponent))
  (if (>= AxisValue 0.0)
    (Class|ChaosVehicleMovementComponent|SetThrottleInput _vehiclemovementcomponent AxisValue)
    (Class|ChaosVehicleMovementComponent|SetBrakeInput _vehiclemovementcomponent 0.0)
    (else
      (Class|ChaosVehicleMovementComponent|SetThrottleInput _vehiclemovementcomponent 0.0)
      (Class|ChaosVehicleMovementComponent|SetBrakeInput _vehiclemovementcomponent (* AxisValue -1.0)))))

(event Input|AxisEvents|InputAxisSteer
  (params (AxisValue :type Float%20%28single-precision%29))
  (Class|ChaosVehicleMovementComponent|SetSteeringInput (Variables|Default|GetVehicleMovementComponent) AxisValue))

(event Input|AxisEvents|InputAxisLookRight
  (params (AxisValue :type Float%20%28single-precision%29))
  (Transformation|AddRelativeRotation (Variables|Default|GetSpringArm) (Math|Rotator|MakeRotator 0.0 0.0 AxisValue) false false))

(event Input|AxisEvents|InputAxisLookUp
  (params (AxisValue :type Float%20%28single-precision%29))
  (Transformation|AddRelativeRotation (Variables|Default|GetSpringArm) (Math|Rotator|MakeRotator 0.0 AxisValue 0.0) false false))

(fn ConstructionScript)