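; BP_Firetruck2 is a drivable firetruck that the player enters and exits by interacting, with possession swapping between character and truck.
; Throttle and steering inputs ease speed and steering angle, which Tick turns into manual, unswept actor offsets and speed-scaled yaw.
; Look inputs rotate the spring arm, while Up and Down scrub a timeline that pitches the ladder.
; Entering hides the interactor; exiting restores it at the truck's mesh and zeroes movement.
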(event EventBeginPlay)

(event Collision|EventActorBeginOverlap
  (params (OtherActor :type Actor%20Object%20Reference)))

(event EventTick
  (params (DeltaSeconds :type Float%20%28single-precision%29))
  (bind _currentspeed (Variables|Default|GetCurrentSpeed))
  (Transformation|AddActorWorldOffset (* DeltaSeconds (* (Transformation|GetActorForwardVector) _currentspeed)))
  (Class|Actor|AddActorWorldRotation (Math|Rotator|MakeRotator 0.0 0.0 (* _currentspeed (Variables|Default|GetCurrentSteeringAngle) (Variables|Default|GetSpeedToRotaationFactor) (Utilities|Time|GetWorldDeltaSeconds)))))

(event EventInteractbyInteracting
  (params (Interactor :type Character%20Object%20Reference))
  (Rendering|SetActorHiddenInGame Interactor true)
  (Collision|SetActorEnableCollision Interactor false)
  (Pawn|Possess (Game|GetPlayerController 0) self))

(event Input|ActionEvents|InputActionInteract
  (params (Key :type Key%20Structure :default "None"))
  (bind _skeletalmesh (Variables|Default|GetSkeletalMesh))
  (:Pressed
    (Transformation|SetActorLocation (stale EventInteractbyInteracting Interactor) (Transformation|GetWorldLocation _skeletalmesh) false true)
    (Transformation|SetActorRotation (stale EventInteractbyInteracting Interactor) (Transformation|GetWorldRotation _skeletalmesh) true)
    (Rendering|SetActorHiddenInGame (stale EventInteractbyInteracting Interactor) false)
    (Collision|SetActorEnableCollision (stale EventInteractbyInteracting Interactor) true)
    (Pawn|Possess (Game|GetPlayerController 0) (stale EventInteractbyInteracting Interactor))
    (Variables|Default|SetCurrentSpeed 0.0)
    (Variables|Default|SetCurrentSteeringAngle 0.0)))

(event Input|ActionEvents|InputActionUp
  (params (Key :type Key%20Structure :default "None"))
  (:Pressed
    (bind _laddermove (Timeline|LadderUp Play)
      (:Update
        (Transformation|SetRelativeRotation (Variables|Default|GetLadder) (Math|Rotator|Lerp(Rotator) "0, 0, 0" "0, 0,-30.000000" _laddermove) false false))))
  (:Released
    (Timeline|LadderUp Stop)))

(event Input|ActionEvents|InputActionDown
  (params (Key :type Key%20Structure :default "None"))
  (:Pressed
    (bind _laddermove (Timeline|LadderUp Reverse)
      (:Update
        (Transformation|SetRelativeRotation (Variables|Default|GetLadder) (Math|Rotator|Lerp(Rotator) "0, 0, 0" "0, 0,-30.000000" _laddermove) false false))))
  (:Released
    (Timeline|LadderUp Stop)))

(event Input|AxisEvents|InputAxisThrottle
  (params (AxisValue :type Float%20%28single-precision%29))
  (Variables|Default|SetCurrentSpeed (Math|Interpolation|FInterpTo (Variables|Default|GetCurrentSpeed) (* AxisValue (Variables|Default|GetMaxSpeed)) (Utilities|Time|GetWorldDeltaSeconds) 4.0)))

(event Input|AxisEvents|InputAxisSteer
  (params (AxisValue :type Float%20%28single-precision%29))
  (Variables|Default|SetCurrentSteeringAngle (Math|Interpolation|FInterpTo (Variables|Default|GetCurrentSteeringAngle) (* AxisValue (Variables|Default|GetMaxSteeringAngle)) (Utilities|Time|GetWorldDeltaSeconds) 4.0)))

(event Input|AxisEvents|InputAxisLookRight
  (params (AxisValue :type Float%20%28single-precision%29))
  (Transformation|AddRelativeRotation (Variables|Default|GetSpringArm) (Math|Rotator|MakeRotator 0.0 0.0 AxisValue) false false))

(event Input|AxisEvents|InputAxisLookUp
  (params (AxisValue :type Float%20%28single-precision%29))
  (Transformation|AddRelativeRotation (Variables|Default|GetSpringArm) (Math|Rotator|MakeRotator 0.0 AxisValue 0.0) false false))

(fn ConstructionScript)