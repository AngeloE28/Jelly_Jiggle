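; Drivable firetruck vehicle Blueprint that turns Steer and Throttle axis input into vehicle movement.
; Steer feeds the VehicleMovementComponent's steering input directly.
; The sign of Throttle splits it into throttle or brake, zeroing the other input so one axis handles both.
; BeginPlay also runs a "PXCIS collision" console command, which looks like a misspelling of the PhysX "pxvis collision" debug view.
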(event EventBeginPlay
  (Development|ExecuteConsoleCommand "PXCIS collision" 0))

(event Collision|EventActorBeginOverlap
  (params (OtherActor :type Actor%20Object%20Reference)))

(event EventTick
  (params (DeltaSeconds :type Float%20%28single-precision%29)))

(event Input|AxisEvents|InputAxisThrottle
  (params (AxisValue :type Float%20%28single-precision%29))
  (bind _vehiclemovementcomponent (Variables|Default|GetVehicleMovementComponent))
  (if (>= AxisValue 0.0)
    (Class|ChaosVehicleMovementComponent|SetThrottleInput _vehiclemovementcomponent AxisValue)
    (Class|ChaosVehicleMovementComponent|SetBrakeInput _vehiclemovementcomponent 0.0)
    (else
      (Class|ChaosVehicleMovementComponent|SetThrottleInput _vehiclemovementcomponent 0.0)
      (Class|ChaosVehicleMovementComponent|SetBrakeInput _vehiclemovementcomponent (* AxisValue -1.0)))))

(event Input|AxisEvents|InputAxisSteer
  (params (AxisValue :type Float%20%28single-precision%29))
  (Class|ChaosVehicleMovementComponent|SetSteeringInput (Variables|Default|GetVehicleMovementComponent) AxisValue))

(fn ConstructionScript)