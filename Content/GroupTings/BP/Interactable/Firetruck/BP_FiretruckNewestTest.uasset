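; A drivable firetruck vehicle pawn with a raisable ladder, entered by interacting with it.
; Interacting hides the interactor, disables its collision and has player controller 0 possess the truck; no exit is implemented.
; Axis inputs feed steering, throttle and brake (negative throttle) to the vehicle movement component and rotate the spring arm camera.
; Held Up/Down inputs play or reverse a timeline that lerps the ladder's pitch, stopping it on release.
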(event EventBeginPlay)

(event Collision|EventActorBeginOverlap
  (params (OtherActor :type Actor%20Object%20Reference)))

(event EventTick
  (params (DeltaSeconds :type Float%20%28single-precision%29)))

(event EventInteractbyInteracting
  (params (Interactor :type Character%20Object%20Reference))
  (Rendering|SetActorHiddenInGame Interactor true)
  (Collision|SetActorEnableCollision Interactor false)
  (Pawn|Possess (Game|GetPlayerController 0) self))

(event Input|ActionEvents|InputActionUp
  (params (Key :type Key%20Structure :default "None"))
  (:Pressed
    (bind _laddermove (Timeline|Timeline_0 Play)
      (:Update
        (Transformation|SetRelativeRotation (Variables|Default|GetLadder) (Math|Rotator|Lerp(Rotator) "0,-90.000000, 0" "0,-90.000000,-30.000000" _laddermove) false false))))
  (:Released
    (Timeline|Timeline_0 Stop)))

(event Input|ActionEvents|InputActionDown
  (params (Key :type Key%20Structure :default "None"))
  (:Pressed
    (bind _laddermove (Timeline|Timeline_0 Reverse)
      (:Update
        (Transformation|SetRelativeRotation (Variables|Default|GetLadder) (Math|Rotator|Lerp(Rotator) "0,-90.000000, 0" "0,-90.000000,-30.000000" _laddermove) false false))))
  (:Released
    (Timeline|Timeline_0 Stop)))

(event Input|AxisEvents|InputAxisThrottle
  (params (AxisValue :type Float%20%28single-precision%29))
  (bind _vehiclemovementcomponent (Variables|Default|GetVehicleMovementComponent))
  (if (>= AxisValue 0.0)
    (Class|ChaosVehicleMovementComponent|SetThrottleInput _vehiclemovementcomponent AxisValue)
    (Class|ChaosVehicleMovementComponent|SetBrakeInput _vehiclemovementcomponent 0.0)
    (else
      (Class|ChaosVehicleMovementComponent|SetThrottleInput _vehiclemovementcomponent 0.0)
      (Class|ChaosVehicleMovementComponent|SetBrakeInput _vehiclemovementcomponent (* AxisValue -1.0)))))

(event Input|AxisEvents|InputAxisSteer
  (params (AxisValue :type Float%20%28single-precision%29))
  (Class|ChaosVehicleMovementComponent|SetSteeringInput (Variables|Default|GetVehicleMovementComponent) AxisValue))

(event Input|AxisEvents|InputAxisLookRight
  (params (AxisValue :type Float%20%28single-precision%29))
  (Transformation|AddRelativeRotation (Variables|Default|GetSpringArm) (Math|Rotator|MakeRotator 0.0 0.0 AxisValue) false false))

(event Input|AxisEvents|InputAxisLookUp
  (params (AxisValue :type Float%20%28single-precision%29))
  (Transformation|AddRelativeRotation (Variables|Default|GetSpringArm) (Math|Rotator|MakeRotator 0.0 AxisValue 0.0) false false))

(fn ConstructionScript)