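; Breakable plate interactable that plays a shatter sound when it fractures under Chaos physics.
; On BeginPlay it adds a Geometry Collection component at a stored plate transform and binds its Chaos break event.
; The break handler plays the sound at that stored location, then gates replays behind a short delayed cooldown so multiple break events do not stack audio.
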(event Custom|PlateBreak
  (params (BreakEvent :type Chaos%20Break%20Event%20Structure%20%28by%20ref%29))
  (if (Variables|Default|GetCanPlaySound?)
    (Audio|PlaySoundatLocation "/Game/GroupTings/SFX/Interactibles/SC_PlateBreak.SC_PlateBreak" (Variables|Default|GetPlateLocation) "0, 0, 0" 1.0 1.0 0.0 0 0 0 0)
    (Variables|Default|SetCanPlaySound? false)
    (Utilities|FlowControl|Delay 3.0)
    (Variables|Default|SetCanPlaySound? true)))

(event EventBeginPlay
  (bind _returnvalue (AddComponent|AddGeometryCollectionComponent false (Math|Transform|MakeTransform (Variables|Default|GetPlateLocation) (Variables|Default|GetPlateRotation) (Variables|Default|GetPlateScale))))
  (Variables|Default|SetPlate1 _returnvalue)
  (EventDispatchers|BindEventtoOnChaosBreakEvent (Variables|Default|GetPlate1) (delegate Custom|PlateBreak)))

(event Collision|EventActorBeginOverlap
  (params (OtherActor :type Actor%20Object%20Reference)))

(event EventTick
  (params (DeltaSeconds :type Float%20%28single-precision%29)))

(fn ConstructionScript)