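; Fire hazard that shrinks interactable actors (BPI_Interact) lingering in its heat, and sends them DeathMessage when they get too small.
; A map holds each actor's time inside, melt threshold and shrink rate, which Tick uses to scale actors down once past their threshold.
; HeatRadius adds and removes entries, HeatedPlatformCollider swaps their rate and threshold while preserving elapsed time, and FireCollider triggers DeathMessage immediately.
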(event OnComponentBeginOverlap(HeatRadius)
  (params (OverlappedComponent :type Primitive%20Component%20Object%20Reference) (OtherActor :type Actor%20Object%20Reference) (OtherComp :type Primitive%20Component%20Object%20Reference) (OtherBodyIndex :type Integer) (bFromSweep :type Boolean) (SweepResult :type Hit%20Result%20Structure%20%28by%20ref%29))
  (if (Utilities|DoesObjectImplementInterface OtherActor "/Game/GroupTings/BP/Interface/BPI_Interact.BPI_Interact_C")
    (if (not (Utilities|Map|Contains (Variables|Default|GetActorsInteracted) OtherActor))
      (Utilities|Map|Add (Variables|Default|GetActorsInteracted) OtherActor (Utilities|Struct|MakeFireInteractionData (Variables|Default|GetscaleDecrement) 0.0 (Variables|Default|GetfireRadiusTimeThreshold))))))

(event OnComponentEndOverlap(HeatRadius)
  (params (OverlappedComponent :type Primitive%20Component%20Object%20Reference) (OtherActor :type Actor%20Object%20Reference) (OtherComp :type Primitive%20Component%20Object%20Reference) (OtherBodyIndex :type Integer))
  (CallFunction|RemoveActorfromMap OtherActor))

(event OnComponentBeginOverlap(FireCollider)
  (params (OverlappedComponent :type Primitive%20Component%20Object%20Reference) (OtherActor :type Actor%20Object%20Reference) (OtherComp :type Primitive%20Component%20Object%20Reference) (OtherBodyIndex :type Integer) (bFromSweep :type Boolean) (SweepResult :type Hit%20Result%20Structure%20%28by%20ref%29))
  (if (Utilities|DoesObjectImplementInterface OtherActor "/Game/GroupTings/BP/Interface/BPI_Interact.BPI_Interact_C")
    (Class|BPIDeath|Death(Message) OtherActor)
    (CallFunction|RemoveActorfromMap OtherActor)))

(event OnComponentBeginOverlap(HeatedPlatformCollider)
  (params (OverlappedComponent :type Primitive%20Component%20Object%20Reference) (OtherActor :type Actor%20Object%20Reference) (OtherComp :type Primitive%20Component%20Object%20Reference) (OtherBodyIndex :type Integer) (bFromSweep :type Boolean) (SweepResult :type Hit%20Result%20Structure%20%28by%20ref%29))
  (bind _actorsinteracted (Variables|Default|GetActorsInteracted))
  (bind (_value _returnvalue) (Utilities|Map|Find _actorsinteracted OtherActor))
  (if _returnvalue
    (Utilities|Map|Add (Variables|Default|GetActorsInteracted) OtherActor (Utilities|Struct|MakeFireInteractionData (Variables|Default|GetheatedPlatformDecrement) (.timeinside _value) (Variables|Default|GetheatedPlatformTimeThreshold)))))

(event OnComponentEndOverlap(HeatedPlatformCollider)
  (params (OverlappedComponent :type Primitive%20Component%20Object%20Reference) (OtherActor :type Actor%20Object%20Reference) (OtherComp :type Primitive%20Component%20Object%20Reference) (OtherBodyIndex :type Integer))
  (bind _actorsinteracted (Variables|Default|GetActorsInteracted))
  (bind (_value _returnvalue) (Utilities|Map|Find _actorsinteracted OtherActor))
  (if _returnvalue
    (Utilities|Map|Add (Variables|Default|GetActorsInteracted) OtherActor (Utilities|Struct|MakeFireInteractionData (Variables|Default|GetscaleDecrement) (.timeinside _value) (Variables|Default|GetfireRadiusTimeThreshold)))))

(event EventTick
  (params (DeltaSeconds :type Float%20%28single-precision%29))
  (if (Utilities|Map|IsNotEmpty (Variables|Default|GetActorsInteracted))
    (bind _keys (Utilities|Map|Keys (Variables|Default|GetActorsInteracted)))
    (for _array_element _keys
      (Utilities|IsValid _array_element
        (:Is%20Valid
          (bind _output_get (Variables|Default|SetcurrentActorInteracted _array_element))
          (bind _returnvalue (CallFunction|2DPLimit(Float) (+ (.timeinside (.Value (Utilities|Map|Find (Variables|Default|GetActorsInteracted) _array_element))) (Utilities|Time|GetWorldDeltaSeconds))))
          (Utilities|Map|Add (Variables|Default|GetActorsInteracted) _output_get (Utilities|Struct|MakeFireInteractionData (.decrementvalue (.Value (Utilities|Map|Find (Variables|Default|GetActorsInteracted) _array_element))) _returnvalue (.melttimethreshold (.Value (Utilities|Map|Find (Variables|Default|GetActorsInteracted) _array_element)))))
          (if (and (.ReturnValue (Utilities|Map|Find (Variables|Default|GetActorsInteracted) (Variables|Default|GetcurrentActorInteracted))) (> (.timeinside (.Value (Utilities|Map|Find (Variables|Default|GetActorsInteracted) (Variables|Default|GetcurrentActorInteracted)))) (.melttimethreshold (.Value (Utilities|Map|Find (Variables|Default|GetActorsInteracted) (Variables|Default|GetcurrentActorInteracted))))))
            (Transformation|SetWorldScale3D (Variables|/Script/Engine.Actor|GetRootComponent (Variables|Default|GetcurrentActorInteracted)) (- (Transformation|GetWorldScale (Variables|/Script/Engine.Actor|GetRootComponent (Variables|Default|GetcurrentActorInteracted))) (* (Utilities|Time|GetWorldDeltaSeconds) (.decrementvalue (.Value (Utilities|Map|Find (Variables|Default|GetActorsInteracted) (Variables|Default|GetcurrentActorInteracted)))))))
            (if (< (.x (Transformation|GetWorldScale (Variables|/Script/Engine.Actor|GetRootComponent (Variables|Default|GetcurrentActorInteracted)))) (Variables|Default|GetsizeLimitToDie))
              (Class|BPIDeath|Death(Message) (Variables|Default|GetcurrentActorInteracted))
              (CallFunction|RemoveActorfromMap (Variables|Default|GetcurrentActorInteracted)))))
        (:Is%20Not%20Valid
          (Utilities|Map|Remove (Variables|Default|GetActorsInteracted) _array_element))))))

(fn ConstructionScript)

(fn RemoveActorfromMap
  (params (currentInteractedActor :type Actor%20Object%20Reference))
  (if (Utilities|Map|Contains (Variables|Default|GetActorsInteracted) currentInteractedActor)
    (Utilities|Map|Remove (Variables|Default|GetActorsInteracted) currentInteractedActor)))