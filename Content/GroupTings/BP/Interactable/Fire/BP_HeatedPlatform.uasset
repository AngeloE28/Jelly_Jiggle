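; Heated platform hazard that shrinks interactable actors standing on it until they die.
; Overlapping BPI_Interact actors, except hats, enter a timer map and get a steam effect in a parallel array.
; Tick accumulates each timer; past the threshold, it moves the steam and shrinks the actor, sending DeathMessage below the size limit.
; Exit or death removes steam by the last ticked index; the game mode's player-death event clears everything.
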(event OnComponentBeginOverlap(HeatedPlatformCollider)
  (params (OverlappedComponent :type Primitive%20Component%20Object%20Reference) (OtherActor :type Actor%20Object%20Reference) (OtherComp :type Primitive%20Component%20Object%20Reference) (OtherBodyIndex :type Integer) (bFromSweep :type Boolean) (SweepResult :type Hit%20Result%20Structure%20%28by%20ref%29))
  (Utilities|Casting|CastToBP_Hat OtherActor
    (:CastFailed
      (if (Utilities|DoesObjectImplementInterface OtherActor "/Game/GroupTings/BP/Interface/BPI_Interact.BPI_Interact_C")
        (if (not (Utilities|Map|Contains (Variables|Default|GetActorsInteracted) OtherActor))
          (Utilities|Map|Add (Variables|Default|GetActorsInteracted) OtherActor (Utilities|Struct|MakeFireInteractionData (Variables|Default|GetscaleDecrement) 0.0 (Variables|Default|GetheatedPlatformTimeThreshold)))
          (bind _returnvalue (Game|SpawnActorfromClass "/Game/StarterContent/Blueprints/Blueprint_Effect_Steam.Blueprint_Effect_Steam_C" (Math|Transform|MakeTransform (Transformation|GetWorldLocation OtherComp) "0, 0, 0" "0.000000,0.000000,0.000000") "Undefined" 0 0))
          (Utilities|Array|Add (Variables|Default|GetfireFeedback) _returnvalue))))))

(event OnComponentEndOverlap(HeatedPlatformCollider)
  (params (OverlappedComponent :type Primitive%20Component%20Object%20Reference) (OtherActor :type Actor%20Object%20Reference) (OtherComp :type Primitive%20Component%20Object%20Reference) (OtherBodyIndex :type Integer))
  (CallFunction|RemoveActorfromMap OtherActor))

(event Custom|PlayerDied
  (params (Character :type Character%20Object%20Reference))
  (bind _firefeedback (Variables|Default|GetfireFeedback))
  (Utilities|Map|Clear (Variables|Default|GetActorsInteracted))
  (for _array_element _firefeedback
    (Actor|DestroyActor _array_element))
  (Utilities|Array|Clear _firefeedback))

(event EventBeginPlay
  (bind _asbp_third_person_game_mode (Utilities|Casting|CastToBP_ThirdPersonGameMode (Game|GetGameMode)))
  (EventDispatchers|BindEventtoOnPlayerDied _asbp_third_person_game_mode (delegate Custom|PlayerDied)))

(event EventTick
  (params (DeltaSeconds :type Float%20%28single-precision%29))
  (if (Utilities|Map|IsNotEmpty (Variables|Default|GetActorsInteracted))
    (bind _keys (Utilities|Map|Keys (Variables|Default|GetActorsInteracted)))
    (for (_array_element _array_index) _keys
      (Variables|Default|SetcurrentArrayIndex _array_index)
      (Utilities|IsValid _array_element
        (:Is%20Valid
          (bind _output_get (Variables|Default|SetcurrentActorInteracted _array_element))
          (bind _returnvalue (CallFunction|2DPLimit(Float) (+ (.timeinside (.Value (Utilities|Map|Find (Variables|Default|GetActorsInteracted) _array_element))) (Utilities|Time|GetWorldDeltaSeconds))))
          (Utilities|Map|Add (Variables|Default|GetActorsInteracted) _output_get (Utilities|Struct|MakeFireInteractionData (.decrementvalue (.Value (Utilities|Map|Find (Variables|Default|GetActorsInteracted) _array_element))) _returnvalue (.melttimethreshold (.Value (Utilities|Map|Find (Variables|Default|GetActorsInteracted) _array_element)))))
          (if (and (> (.timeinside (.Value (Utilities|Map|Find (Variables|Default|GetActorsInteracted) (Variables|Default|GetcurrentActorInteracted)))) (.melttimethreshold (.Value (Utilities|Map|Find (Variables|Default|GetActorsInteracted) (Variables|Default|GetcurrentActorInteracted))))) (.ReturnValue (Utilities|Map|Find (Variables|Default|GetActorsInteracted) (Variables|Default|GetcurrentActorInteracted))))
            (bind _currentactorinteracted (Variables|Default|GetcurrentActorInteracted)
              (:then
                (Transformation|SetActorLocation (Utilities|Array|Get(acopy) (Variables|Default|GetfireFeedback) (Variables|Default|GetcurrentArrayIndex)) (Transformation|GetWorldLocation (Utilities|Array|Get(acopy) (Components|GetChildrenComponents (Variables|/Script/Engine.Actor|GetRootComponent _currentactorinteracted) false))) false false)
                (Utilities|FlowControl|Sequence
                  (:then_0
                    (Transformation|SetWorldScale3D (Variables|/Script/Engine.Actor|GetRootComponent _currentactorinteracted) (- (Transformation|GetWorldScale (Variables|/Script/Engine.Actor|GetRootComponent _currentactorinteracted)) (* (Utilities|Time|GetWorldDeltaSeconds) (.decrementvalue (.Value (Utilities|Map|Find (Variables|Default|GetActorsInteracted) (Variables|Default|GetcurrentActorInteracted)))))))
                    (if (< (.x (Transformation|GetWorldScale (Variables|/Script/Engine.Actor|GetRootComponent (Variables|Default|GetcurrentActorInteracted)))) (Variables|Default|GetsizeLimitToDie))
                      (Class|BPIDeath|Death(Message) (Variables|Default|GetcurrentActorInteracted))
                      (CallFunction|RemoveActorfromMap (Variables|Default|GetcurrentActorInteracted))))))
              (:else))))
        (:Is%20Not%20Valid
          (Utilities|Map|Remove (Variables|Default|GetActorsInteracted) _array_element))))))

(fn ConstructionScript)

(fn RemoveActorfromMap
  (params (currentInteractedActor :type Actor%20Object%20Reference))
  (if (Utilities|Map|Contains (Variables|Default|GetActorsInteracted) currentInteractedActor)
    (Utilities|Map|Remove (Variables|Default|GetActorsInteracted) currentInteractedActor)
    (bind _asblueprint_effect_steam (Utilities|Casting|CastToBlueprint_Effect_Steam (Utilities|Array|Get(acopy) (Variables|Default|GetfireFeedback) (Variables|Default|GetcurrentArrayIndex))))
    (Default|KillSteam _asblueprint_effect_steam)
    (Utilities|Array|RemoveIndex (Variables|Default|GetfireFeedback) (Variables|Default|GetcurrentArrayIndex))))