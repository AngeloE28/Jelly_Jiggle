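; Interactable microwave that traps and kills Characters who stay inside too long.
; Tick times occupancy of DeathCollider; past the limit it swings the door shut, scales up a blocking collider, then after a delay calls DeathMessage on occupants and clears the blocker.
; An interactable actor overlapping OpenDoorCollider while the door is closed re-arms a DoOnce, which resets itself each tick to interpolate the door open.
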(event OnComponentBeginOverlap(openDoorCollider)
  (params (OverlappedComponent :type Primitive%20Component%20Object%20Reference) (OtherActor :type Actor%20Object%20Reference) (OtherComp :type Primitive%20Component%20Object%20Reference) (OtherBodyIndex :type Integer) (bFromSweep :type Boolean) (SweepResult :type Hit%20Result%20Structure%20%28by%20ref%29))
  (bind _door (Variables|Default|Getdoor))
  (bind _returnvalue (Transformation|GetWorldRotation _door))
  (if (and (Utilities|DoesObjectImplementInterface OtherActor "/Game/GroupTings/BP/Interface/BPI_Interact.BPI_Interact_C") (< (- (.yaw (Transformation|GetWorldRotation (Variables|Default|Getdoor))) (.yaw (Transformation|GetActorRotation))) (Variables|Default|GetclosedDoorLimit)))
    (Utilities|FlowControl|DoOnce true) ; enters at Reset
  ))

(event OnComponentBeginOverlap(deathCollider)
  (params (OverlappedComponent :type Primitive%20Component%20Object%20Reference) (OtherActor :type Actor%20Object%20Reference) (OtherComp :type Primitive%20Component%20Object%20Reference) (OtherBodyIndex :type Integer) (bFromSweep :type Boolean) (SweepResult :type Hit%20Result%20Structure%20%28by%20ref%29))
  (if (Utilities|ClassIsChildOf (Utilities|GetClass OtherActor) "/Script/Engine.Character")
    (Variables|Default|SettimeInside 0.0)))

(event EventTick
  (params (DeltaSeconds :type Float%20%28single-precision%29))
  (bind _door (Variables|Default|Getdoor))
  (bind _door_2 (Variables|Default|Getdoor))
  (bind _returnvalue (Transformation|GetWorldRotation _door_2))
  (bind _returnvalue_2 (Transformation|GetWorldRotation _door))
  (Utilities|FlowControl|Sequence
    (:then_0
      (if (Utilities|Array|IsNotEmpty (Collision|GetOverlappingActors (Variables|Default|GetdeathCollider) "/Script/Engine.Character" :!class /Script/Engine.PrimitiveComponent))
        (bind _returnvalue_3 (CallFunction|2DPLimit(Float) (+ (Variables|Default|GettimeInside) (Utilities|Time|GetWorldDeltaSeconds))))
        (bind _output_get (Variables|Default|SettimeInside _returnvalue_3))
        (if (> _output_get (Variables|Default|GettimeToKillPlayer))
          (Transformation|SetWorldRotation _door_2 (Math|Rotator|MakeRotator (.roll _returnvalue) (.pitch _returnvalue) (Math|Interpolation|FInterpTo (.yaw _returnvalue) (.yaw (Transformation|GetActorRotation)) (Utilities|Time|GetWorldDeltaSeconds) (Variables|Default|GetdoorAnimSpeed))) false false)
          (Transformation|SetWorldScale3D (Variables|Default|GetblockingCollider) (* (Variables|Default|GetdoorScale) (Transformation|GetActorScale3D)))
          (Utilities|FlowControl|Delay (Variables|Default|GetplayerDeathDelay))
          (for _array_element (Collision|GetOverlappingActors (Variables|Default|GetdeathCollider) "/Script/Engine.Character" :!class /Script/Engine.PrimitiveComponent)
            (Utilities|IsValid _array_element
              (:Is%20Valid
                (Class|BPIDeath|Death(Message) _array_element)
                (Variables|/Game/GroupTings/BP/Dialogue/BP_NPC.BP_NPC_C|SetResetJelly (Variables|Default|GetBP_NPC) false))))
          (Transformation|SetWorldScale3D (Variables|Default|GetblockingCollider) "0, 0, 0")
          (Variables|Default|SettimeInside 0.0))))
    (:then_1
      (Utilities|FlowControl|DoOnce true :!label _label
        (:Completed
          (Transformation|SetWorldRotation _door (Math|Rotator|MakeRotator (.roll _returnvalue_2) (.pitch _returnvalue_2) (Math|Interpolation|FInterpTo (.yaw _returnvalue_2) (+ (Variables|Default|GetdoorRotationWhenOpened) (.yaw (Transformation|GetActorRotation))) (Utilities|Time|GetWorldDeltaSeconds) (Variables|Default|GetdoorAnimSpeed))) false false)
          (if (< (- (.yaw (Transformation|GetWorldRotation (Variables|Default|Getdoor))) (.yaw (Transformation|GetActorRotation))) (Variables|Default|GetopenDoorLimit))
            (goto _label Reset)))))))

(fn ConstructionScript)