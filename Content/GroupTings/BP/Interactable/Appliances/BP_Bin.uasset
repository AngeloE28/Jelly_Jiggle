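; BP_Bin is an interactable pedal bin that opens when stepped on and launches the character upward when they leave the pedal.
; PedalCollider overlaps with BPI_Interact actors set OverlappingPlayer, and Tick eases Foot and Lid between idle and stepped-on world rotations with RInterpTo.
; BeginPlay builds those rotations from the actor's roll and yaw plus each variable's preset pitch.
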(event OnComponentBeginOverlap(pedalCollider)
  (params (OverlappedComponent :type Primitive%20Component%20Object%20Reference) (OtherActor :type Actor%20Object%20Reference) (OtherComp :type Primitive%20Component%20Object%20Reference) (OtherBodyIndex :type Integer) (bFromSweep :type Boolean) (SweepResult :type Hit%20Result%20Structure%20%28by%20ref%29))
  (if (Utilities|DoesObjectImplementInterface OtherActor "/Game/GroupTings/BP/Interface/BPI_Interact.BPI_Interact_C")
    (Variables|Default|SetoverlappingPlayer true)))

(event OnComponentEndOverlap(pedalCollider)
  (params (OverlappedComponent :type Primitive%20Component%20Object%20Reference) (OtherActor :type Actor%20Object%20Reference) (OtherComp :type Primitive%20Component%20Object%20Reference) (OtherBodyIndex :type Integer))
  (if (Utilities|DoesObjectImplementInterface OtherActor "/Game/GroupTings/BP/Interface/BPI_Interact.BPI_Interact_C")
    (Variables|Default|SetoverlappingPlayer false)
    (bind _ascharacter (Utilities|Casting|CastToCharacter OtherActor))
    (Character|LaunchCharacter _ascharacter "0, 0,2000.000000" false false)))

(event EventTick
  (params (DeltaSeconds :type Float%20%28single-precision%29))
  (bind _lid (Variables|Default|Getlid))
  (bind _foot (Variables|Default|Getfoot))
  (bind _lid_2 (Variables|Default|Getlid))
  (bind _foot_2 (Variables|Default|Getfoot))
  (if (Variables|Default|GetoverlappingPlayer)
    (Transformation|SetWorldRotation _foot (Math|Interpolation|RInterpTo (Transformation|GetWorldRotation _foot) (Variables|Default|GetsteppedOnRotation%28foot%29) (Utilities|Time|GetWorldDeltaSeconds) (Variables|Default|GetInterp%20Speed%28foot%29)) false false)
    (Transformation|SetWorldRotation _lid (Math|Interpolation|RInterpTo (Transformation|GetWorldRotation _lid) (Variables|Default|GetsteppedOnRotation%28lid%29) (Utilities|Time|GetWorldDeltaSeconds) (Variables|Default|GetInterp%20Speed%28lid%29)) false false)
    (else
      (Transformation|SetWorldRotation _foot_2 (Math|Interpolation|RInterpTo (Transformation|GetWorldRotation _foot_2) (Variables|Default|GetidleRotation%28foot%29) (Utilities|Time|GetWorldDeltaSeconds) (Variables|Default|GetInterp%20Speed%28foot%29)) false false)
      (Transformation|SetWorldRotation _lid_2 (Math|Interpolation|RInterpTo (Transformation|GetWorldRotation _lid_2) (Variables|Default|GetidleRotation%28lid%29) (Utilities|Time|GetWorldDeltaSeconds) (Variables|Default|GetInterp%20Speed%28lid%29)) false false))))

(event EventBeginPlay
  (bind _returnvalue (Transformation|GetActorRotation))
  (bind _output_get (Variables|Default|SetidleRotation%28foot%29 (Math|Rotator|MakeRotator (.roll _returnvalue) (.pitch (Variables|Default|GetidleRotation%28foot%29)) (.yaw _returnvalue))))
  (bind _output_get_2 (Variables|Default|SetidleRotation%28lid%29 (Math|Rotator|MakeRotator (.roll _output_get) (.pitch (Variables|Default|GetidleRotation%28lid%29)) (.yaw _output_get))))
  (bind _output_get_3 (Variables|Default|SetsteppedOnRotation%28foot%29 (Math|Rotator|MakeRotator (.roll _output_get_2) (.pitch (Variables|Default|GetsteppedOnRotation%28foot%29)) (.yaw _output_get_2))))
  (Variables|Default|SetsteppedOnRotation%28lid%29 (Math|Rotator|MakeRotator (.roll _output_get_3) (.pitch (Variables|Default|GetsteppedOnRotation%28lid%29)) (.yaw _output_get_3))))

(fn ConstructionScript)