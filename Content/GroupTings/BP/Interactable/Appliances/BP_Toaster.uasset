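; Interactable toaster that works as a launch pad, firing the player straight up when it is shot while a character overlaps it.
; Overlap begin, overlap end and shooting drive a physics constraint's linear position target, with sounds on entry and launch.
; Tick copies the hidden pad's height to the lever and toast launch pieces.
; The first overlap also teleports both bread pieces to that height, once only.
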(event OnComponentBeginOverlap(overlapCollider)
  (params (OverlappedComponent :type Primitive%20Component%20Object%20Reference) (OtherActor :type Actor%20Object%20Reference) (OtherComp :type Primitive%20Component%20Object%20Reference) (OtherBodyIndex :type Integer) (bFromSweep :type Boolean) (SweepResult :type Hit%20Result%20Structure%20%28by%20ref%29))
  (bind _bread (Variables|Default|Getbread))
  (bind _bread2 (Variables|Default|Getbread2))
  (bind _returnvalue (Transformation|GetWorldLocation _bread))
  (bind _returnvalue_2 (Transformation|GetWorldLocation _bread2))
  (if (Utilities|ClassIsChildOf (Utilities|GetClass OtherActor) "/Script/Engine.Character")
    (Variables|Default|SetoveralappingPlayer true)
    (Class|PhysicsConstraintComponent|SetLinearPositionTarget (Variables|Default|GetPhysicsConstraint) (Math|Vector|MakeVector 0.0 0.0 6e+01))
    (Audio|PlaySound2D "/Game/GroupTings/SFX/Toaster/SFX_Toaster1.SFX_Toaster1" 1.0 1.0 0.0 0 0)
    (Utilities|FlowControl|DoOnce false
      (:Completed
        (Transformation|SetWorldLocation _bread2 (Math|Vector|MakeVector (.x _returnvalue_2) (.y _returnvalue_2) (.z (Transformation|GetWorldLocation (Variables|Default|Getpadhidden)))) false true)
        (Transformation|SetWorldLocation _bread (Math|Vector|MakeVector (.x _returnvalue) (.y _returnvalue) (.z (Transformation|GetWorldLocation (Variables|Default|Getpadhidden)))) false true)))))

(event OnComponentEndOverlap(overlapCollider)
  (params (OverlappedComponent :type Primitive%20Component%20Object%20Reference) (OtherActor :type Actor%20Object%20Reference) (OtherComp :type Primitive%20Component%20Object%20Reference) (OtherBodyIndex :type Integer))
  (if (Utilities|ClassIsChildOf (Utilities|GetClass OtherActor) "/Script/Engine.Character")
    (Variables|Default|SetoveralappingPlayer false)
    (Class|PhysicsConstraintComponent|SetLinearPositionTarget (Variables|Default|GetPhysicsConstraint) (Math|Vector|MakeVector 0.0 0.0 0.0))))

(event EventTick
  (params (DeltaSeconds :type Float%20%28single-precision%29))
  (bind _toastlaunch (Variables|Default|GettoastLaunch))
  (bind _lever (Variables|Default|Getlever))
  (bind _toastlaunch1 (Variables|Default|GettoastLaunch1))
  (bind _returnvalue (Transformation|GetWorldLocation _toastlaunch))
  (bind _returnvalue_2 (Transformation|GetWorldLocation _toastlaunch1))
  (bind _returnvalue_3 (Transformation|GetWorldLocation _lever))
  (Transformation|SetWorldLocation _lever (Math|Vector|MakeVector (.x _returnvalue_3) (.y _returnvalue_3) (.z (Transformation|GetWorldLocation (Variables|Default|Getpadhidden)))) false false)
  (Transformation|SetWorldLocation _toastlaunch (Math|Vector|MakeVector (.x _returnvalue) (.y _returnvalue) (.z (Transformation|GetWorldLocation (Variables|Default|Getpadhidden)))) false false)
  (Transformation|SetWorldLocation _toastlaunch1 (Math|Vector|MakeVector (.x _returnvalue_2) (.y _returnvalue_2) (.z (Transformation|GetWorldLocation (Variables|Default|Getpadhidden)))) false false))

(event EventInteractbyShooting
  (if (Variables|Default|GetoveralappingPlayer)
    (Class|PhysicsConstraintComponent|SetLinearPositionTarget (Variables|Default|GetPhysicsConstraint) (Math|Vector|MakeVector 0.0 0.0 -1e+01))
    (Audio|PlaySound2D "/Game/GroupTings/SFX/Toaster/SFX_Toaster2.SFX_Toaster2" 1.0 1.0 0.0 0 0)
    (Character|LaunchCharacter (Game|GetPlayerCharacter 0) "0, 0,2000.000000" false false)))

(fn ConstructionScript)