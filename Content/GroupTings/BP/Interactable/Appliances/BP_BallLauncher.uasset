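; BP_BallLauncher is an interactable appliance that carries a player along a spline and launches them.
; Its collider reacts to a BP_TennisBall attached to a BP_PlayerJelly and starts a timeline whose play rate derives from the air time.
; The timeline moves the player's capsule along the spline and rotates the mesh to match.
; Past a set path threshold, a do-once launches the character along the spline direction and stops the timeline.
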(event OnComponentBeginOverlap(Collider)
  (params (OverlappedComponent :type Primitive%20Component%20Object%20Reference) (OtherActor :type Actor%20Object%20Reference) (OtherComp :type Primitive%20Component%20Object%20Reference) (OtherBodyIndex :type Integer) (bFromSweep :type Boolean) (SweepResult :type Hit%20Result%20Structure%20%28by%20ref%29))
  (bind _asbp_tennis_ball (Utilities|Casting|CastToBP_TennisBall OtherActor))
  (bind _asbp_player_jelly (Utilities|Casting|CastToBP_PlayerJelly (Actor|GetAttachParentActor _asbp_tennis_ball)))
  (CallFunction|MoveAlongPath _asbp_player_jelly))

(event Custom|MoveAlongPath
  (params (Player :type BP%20Player%20Jelly%20Object%20Reference))
  (bind _capsulecomponent (Variables|/Script/Engine.Character|GetCapsuleComponent Player))
  (bind _returnvalue (Transformation|GetWorldTransform _capsulecomponent))
  (Components|Timeline|SetPlayRate (Variables|Default|GetMove_Timeline) (/ 1.0 (Variables|Default|GetPlayerAirTime)))
  (bind _movetrack (Timeline|Move_Timeline PlayFromStart)
    (:Update
      (Transformation|SetWorldTransform _capsulecomponent (Math|Transform|MakeTransform (Spline|GetLocationatDistanceAlongSpline (Variables|Default|GetSpline) (Math|Float|Lerp 0.0 (Spline|GetSplineLength (Variables|Default|GetSpline)) _movetrack) "World") (.rotation _returnvalue) (.scale _returnvalue)) false false)
      (Transformation|SetWorldRotation (Variables|/Script/Engine.Character|GetMesh Player) (Spline|GetRotationatDistanceAlongSpline (Variables|Default|GetSpline) (Math|Float|Lerp 0.0 (Spline|GetSplineLength (Variables|Default|GetSpline)) _movetrack) "World") false false)
      (if (> _movetrack (Variables|Default|GetMaxDistAlongSplinePath))
        (Utilities|FlowControl|DoOnce false :!label _label
          (:Completed
            (Character|LaunchCharacter Player (* (Math|Vector|Normalize (Math|Rotator|GetRotationXVector (Spline|GetRotationatDistanceAlongSpline (Variables|Default|GetSpline) (Math|Float|Lerp 0.0 (Spline|GetSplineLength (Variables|Default|GetSpline)) _movetrack) "World"))) (Variables|Default|GetlaunchStrength)) true false)
            (Timeline|Move_Timeline Stop)))))
    (:Finished
      (goto _label Reset))))

(fn ConstructionScript)