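; Gate trigger that opens a locked gate when an actor tagged "Key" overlaps its trigger volume.
; On BeginPlay it caches the first actor tagged "OpeningGate" as the gate to move.
; The overlap destroys the key, hides the lock mesh and disables its collision, then a timeline rotates the gate open.
; An unlock sound plays once, when the timeline finishes.
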(event OnComponentBeginOverlap(Trigger)
  (params (OverlappedComponent :type Primitive%20Component%20Object%20Reference) (OtherActor :type Actor%20Object%20Reference) (OtherComp :type Primitive%20Component%20Object%20Reference) (OtherBodyIndex :type Integer) (bFromSweep :type Boolean) (SweepResult :type Hit%20Result%20Structure%20%28by%20ref%29))
  (bind _lockmesh (Variables|Default|GetLockMesh))
  (if (Actor|ActorHasTag OtherActor "Key")
    (Actor|DestroyActor OtherActor)
    (Collision|SetCollisionEnabled _lockmesh "NoCollision")
    (Development|SetHiddeninGame _lockmesh true false)
    (bind _move (Timeline|GateOpen Play)
      (:Update
        (Transformation|SetActorRotation (Variables|Default|GetOpenGate) (Math|Rotator|Lerp(Rotator) "0,180.000000, 0" "0,270.000000, 0" _move)))
      (:Finished
        (if (not (Variables|Default|GetSoundPlayed?))
          (Audio|PlaySound2D "/Game/GroupTings/SFX/Interactibles/SC_Unlock.SC_Unlock" 1.0 1.0 0.0 0 0)
          (Variables|Default|SetSoundPlayed? true))))))

(event EventBeginPlay
  (bind _outactors (Actor|GetAllActorswithTag "OpeningGate"))
  (Variables|Default|SetOpenGate (Utilities|Array|Get(acopy) _outactors)))

(fn ConstructionScript)