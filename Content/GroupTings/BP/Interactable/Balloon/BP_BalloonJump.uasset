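; BP_BalloonJump is an interactable balloon that bounces characters touching its mesh and jiggles in response.
; On overlap it launches the Character along the sweep's impact normal, adding to its existing velocity.
; It writes the impact point to the MPC_JiggleData material parameter collection, then a timeline drives a scaled normal vector into that collection.
; Because the collection is global, all materials reading it share the latest jiggle.
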(event OnComponentBeginOverlap(BalloonMesh)
  (params (OverlappedComponent :type Primitive%20Component%20Object%20Reference) (OtherActor :type Actor%20Object%20Reference) (OtherComp :type Primitive%20Component%20Object%20Reference) (OtherBodyIndex :type Integer) (bFromSweep :type Boolean) (SweepResult :type Hit%20Result%20Structure%20%28by%20ref%29))
  (bind (_bblockinghit _binitialoverlap _time _distance _location _impactpoint _normal _impactnormal) (Collision|BreakHitResult SweepResult))
  (if (Utilities|ClassIsChildOf (Utilities|GetClass OtherActor) "/Script/Engine.Character")
    (bind _ascharacter (Utilities|Casting|CastToCharacter OtherActor))
    (Character|LaunchCharacter _ascharacter (* _impactnormal (Variables|Default|GetlaunchStrength)) false false)
    (Rendering|Material|SetVectorParameterValue "/Game/GroupTings/Materials/Jiggle/Data/MPC_JiggleData.MPC_JiggleData" "Position" (Math|Conversions|ToLinearColor(Vector) _impactpoint) :!class /Script/Engine.KismetMaterialLibrary)
    (bind _jiggle_track (Timeline|Jiggle_Timeline PlayFromStart)
      (:Update
        (Rendering|Material|SetVectorParameterValue "/Game/GroupTings/Materials/Jiggle/Data/MPC_JiggleData.MPC_JiggleData" "Normal" (Math|Conversions|ToLinearColor(Vector) (* _impactnormal (* _jiggle_track (Variables|Default|GetjiggleStrength)))) :!class /Script/Engine.KismetMaterialLibrary)))))

(fn ConstructionScript)