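; BP_Dog is an AI-controlled dog character that attacks and kills player and other jelly characters.
; Its attack collider plays an angry sound and an attack montage, toggling attack behaviour on BP_DogController.
; A death collider follows the nose socket every tick, sending DeathMessage to jellies it touches and notifying the controller of player kills.
; Helper functions set walk speed or put it to sleep by disabling movement and both colliders.
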(event OnComponentBeginOverlap(AttackCollider)
  (params (OverlappedComponent :type Primitive%20Component%20Object%20Reference) (OtherActor :type Actor%20Object%20Reference) (OtherComp :type Primitive%20Component%20Object%20Reference) (OtherBodyIndex :type Integer) (bFromSweep :type Boolean) (SweepResult :type Hit%20Result%20Structure%20%28by%20ref%29))
  (if (Utilities|DoesObjectImplementInterface OtherActor "/Game/GroupTings/BP/Interface/BPI_Interact.BPI_Interact_C")
    (Audio|PlaySoundatLocation "/Game/GroupTings/SFX/Dog/SFX_Dog_Angry.SFX_Dog_Angry" (Transformation|GetActorLocation self) "0, 0, 0" 1.0 1.0 0.0 0 "/Game/GroupTings/SFX/SCC_JellyProj.SCC_JellyProj" 0 0)
    (Utilities|Casting|CastToBP_PlayerJelly OtherActor
      (:then
        _)
      (:CastFailed
        (Utilities|Casting|CastToBP_JellyBase OtherActor)))
    (Animation|Montage|PlayMontage (Variables|Character|GetMesh) "/Game/GroupTings/Characters/Dog_Doberman/Animations/Anim_Doberman_Attack_J_Montage.Anim_Doberman_Attack_J_Montage" 1.25
      (:then
        (bind _asbp_dog_controller (Utilities|Casting|CastToBP_DogController (Pawn|GetController)))
        (Default|AttackBehaviour _asbp_dog_controller true))
      (:OnCompleted
        (bind _asbp_dog_controller_2 (Utilities|Casting|CastToBP_DogController (Pawn|GetController)))
        (Default|AttackBehaviour _asbp_dog_controller_2 false)))))

(event OnComponentBeginOverlap(DeathCollider)
  (params (OverlappedComponent :type Primitive%20Component%20Object%20Reference) (OtherActor :type Actor%20Object%20Reference) (OtherComp :type Primitive%20Component%20Object%20Reference) (OtherBodyIndex :type Integer) (bFromSweep :type Boolean) (SweepResult :type Hit%20Result%20Structure%20%28by%20ref%29))
  (if (Utilities|DoesObjectImplementInterface OtherActor "/Game/GroupTings/BP/Interface/BPI_Interact.BPI_Interact_C")
    (Utilities|Casting|CastToBP_PlayerJelly OtherActor
      (:then
        (Utilities|FlowControl|Sequence
          (:then_0
            (Class|BPIDeath|Death(Message) OtherActor :!label _label))
          (:then_1
            (bind _asbp_dog_controller (Utilities|Casting|CastToBP_DogController (Pawn|GetController)))
            (Default|KilledPlayer _asbp_dog_controller))))
      (:CastFailed
        (Utilities|Casting|CastToBP_JellyBase OtherActor)
        (goto _label)))))

(event EventTick
  (params (DeltaSeconds :type Float%20%28single-precision%29))
  (bind _mesh (Variables|Character|GetMesh))
  (bind _nose (Variables|Default|GetNose))
  (Transformation|SetWorldLocationAndRotation (Variables|Default|GetDeathCollider) (Transformation|GetSocketLocation _mesh _nose) (Transformation|GetSocketRotation _mesh _nose) false false))

(event EventBeginPlay
  (Variables|Default|SetisSleep false))

(fn ConstructionScript)

(fn UpdateWalkSpeed
  (params (NewWalkSpeed :type Float%20%28double-precision%29))
  (Variables|/Script/Engine.CharacterMovementComponent|SetMaxWalkSpeed (Variables|Character|GetCharacterMovement) NewWalkSpeed))

(fn Sleep
  (Pawn|Components|CharacterMovement|DisableMovement (Variables|Character|GetCharacterMovement))
  (Variables|Default|SetisSleep true)
  (Collision|SetCollisionEnabled (Variables|Default|GetAttackCollider) "NoCollision")
  (Collision|SetCollisionEnabled (Variables|Default|GetDeathCollider) "NoCollision"))