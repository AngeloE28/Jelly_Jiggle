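; AI controller for the dog that runs BT_Dog on possession and tracks the player jelly through AI perception.
; Sensing the player sets the line-of-sight and enemy blackboard keys, while losing it starts a grace timer that clears them.
; Block and unblock events gate perception updates through a LineOfSight flag.
; Helper functions set the Sleep key or clear the target after a player kill.
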(event OnTargetPerceptionUpdated(AIPerception)
  (params (Actor :type Actor%20Object%20Reference) (Stimulus :type AI%20Stimulus%20Structure))
  (bind _blackboard (Variables|Default|GetBlackboard))
  (if (Variables|Default|GetLineOfSight)
    (bind _asbp_player_jelly (Utilities|Casting|CastToBP_PlayerJelly Actor)
      (:then
        (if (Utilities|Struct|BreakAIStimulus Stimulus)
          (Utilities|Time|ClearandInvalidateTimerbyHandle (Variables|Default|GetEnemyTimer))
          (AI|Components|Blackboard|SetValueasBool _blackboard (Variables|Default|GetHasLineOfSight) true)
          (AI|Components|Blackboard|SetValueasObject _blackboard (Variables|Default|GetEnemyActor) _asbp_player_jelly)
          (else
            (bind _returnvalue (Utilities|Time|SetTimerbyEvent (delegate Custom|StartEnemyTimer) (Variables|Default|GetLineOfSightTimer) :!label _label))
            (Variables|Default|SetEnemyTimer _returnvalue))))
      (:CastFailed
        (goto _label)))))

(event Custom|StartEnemyTimer
  (bind _blackboard (Variables|Default|GetBlackboard))
  (AI|Components|Blackboard|SetValueasBool _blackboard (Variables|Default|GetHasLineOfSight) false)
  (AI|Components|Blackboard|SetValueasObject _blackboard (Variables|Default|GetEnemyActor) 0))

(event EventPossess
  (params (PossessedPawn :type Pawn%20Object%20Reference))
  (AI|RunBehaviorTree "/Game/GroupTings/BP/Interactable/Dog/BT_Dog.BT_Dog"))

(event EventBlockLineOfSight
  (Variables|Default|SetLineOfSight false))

(event EventUnBlockLineOfSight
  (Variables|Default|SetLineOfSight true))

(fn ConstructionScript)

(fn SleepBehaviour
  (AI|Components|Blackboard|SetValueasBool (Variables|Default|GetBlackboard) (Variables|Default|GetSleep) true))

(fn KilledPlayer
  (bind _blackboard (Variables|Default|GetBlackboard))
  (AI|Components|Blackboard|SetValueasBool _blackboard (Variables|Default|GetHasLineOfSight) false)
  (AI|Components|Blackboard|SetValueasObject _blackboard (Variables|Default|GetEnemyActor) 0))